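; Force feedback actor component that overrides its parent's intensity multiplier with the force feedback value stored in the player's saved settings.
; GetIntensityMultiplier gets the settings save game through the GameInstance and returns its force feedback setting, falling back to the parent implementation when that object is invalid.
; The event graph holds only disabled default BeginPlay and Tick nodes.
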(fn `GetIntensityMultiplier`
  (returns (ReturnValue :type "Float (double-precision)"))
  (bind _returnvalue (message `/Game/LelouFW/Blueprint/GameInstance/LelouFW_BPI_GameInstance_Settings_Interface.GetSettingsSaveGame` (`GameplayStatics.GetGameInstance`)))
  (`/Engine/EditorBlueprintResources/StandardMacros.IsValid` _returnvalue
    (:`Is Valid`
      (bind _returnvalue_2 (message `/Game/LelouFW/Blueprint/SaveGame/Settings/LelouFW_BPI_SaveGame_Settings_Interface.GetForceFeedbackSettingsInSaveGame` _returnvalue))
      (return _returnvalue_2))
    (:`Is Not Valid`
      (bind _returnvalue_3 (`parent.GetIntensityMultiplier`))
      (return _returnvalue_3))))