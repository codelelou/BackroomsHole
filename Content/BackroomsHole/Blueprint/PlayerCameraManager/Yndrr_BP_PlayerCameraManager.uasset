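; Player camera manager child class that adds game-specific rules to the parent's camera zoom.
; ValidZoom blocks zooming while the character is falling or a dialogue, save menu, actor viewer or inventory HUD is visible.
; The zoom-changed event stops sprinting and uses DoOnce gates to slow walking during zoom, then restore the speed cached on first zoom.
; FOV changes go to the parent, leaving an older camera-modifier approach disconnected.
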(event `/Game/LelouFW/Blueprint/PlayerCameraManager/LelouFW_BPI_PlayerCameraManager_Interface.SetFOVAtCharacterCamera`
  (params (FOV :type "Float (double-precision)"))
  (`self.SetFOV` FOV))

(event `self.ReceiveBeginPlay`
  (`parent.ReceiveBeginPlay`))

(event `self.SetFOV`
  (params (NewFOV :type "Float (double-precision)"))
  ;[1 1 1] Zoom
  (`parent.SetFOV` NewFOV))

(event `self.CallZoomChangedEventDispatcher`
  (params (Zooming :type Boolean) (Alpha :type "Float (double-precision)") (Direction :type "ETimelineDirection Enum" :default "Forward"))
  ;[1 1 1] Zoom
  (`parent.CallZoomChangedEventDispatcher` Zooming Alpha Direction)
  (`|ExecutionSequence`
    (:`then_0`
      (`/Engine/EditorBlueprintResources/StandardMacros.DoOnce` false :!label _label
        (:`Completed`
          (bind _returnvalue (message `/Game/LelouFW/Blueprint/Controller/LelouFW_BPI_PlayerController_Interface.GetControllerHelper` (`self.GetOwningPlayerController`)))
          (message `/Game/LelouFW/Blueprint/Controller/Helper/LelouFW_BPI_Controller_Character_Interface.StopSprintingAtCharacter` _returnvalue))))
    (:`then_1`
      (if (not Zooming)
        (goto _label :!via `Reset`)))
    (:`then_2`
      (`self.UpdateCharacterSpeedByZooming` Zooming))))

(event `UpdateCharacterSpeedByZooming`
  (params (Zooming :type Boolean))
  (bind _charactermovement (`Character.CharacterMovement` (`GameplayStatics.GetPlayerCharacter` 0)))
  ;[1 1 1] Zoom
  (if Zooming
    (`|ExecutionSequence`
      (:`then_0`
        (`/Engine/EditorBlueprintResources/StandardMacros.DoOnce` false :!label _label_2
          (:`Completed`
            (`|ExecutionSequence`
              (:`then_0`
                (`/Engine/EditorBlueprintResources/StandardMacros.DoOnce` false
                  (:`Completed`
                    (bind _output_get (set `self.CharacterMaxWalkSpeed` (`CharacterMovementComponent.MaxWalkSpeed` _charactermovement))))))
              (:`then_1`
                (set `CharacterMovementComponent.MaxWalkSpeed` 20.0 _charactermovement))))))
      (:`then_1`
        (goto _label_3 :!via `Reset`)))
    (else
      (`|ExecutionSequence`
        (:`then_0`
          (`/Engine/EditorBlueprintResources/StandardMacros.DoOnce` true :!label _label_3
            (:`Completed`
              (set `CharacterMovementComponent.MaxWalkSpeed` _output_get _charactermovement))))
        (:`then_1`
          (goto _label_2 :!via `Reset`))))))

(fn `UserConstructionScript`
  (`parent.UserConstructionScript`))

(fn `ValidZoom`
  (returns (ReturnValue :type Boolean))
  (bind _returnvalue (`PlayerController.GetHUD` (`self.GetOwningPlayerController`)))
  (if (not (`NavMovementComponent.IsFalling` (`Character.CharacterMovement` (`GameplayStatics.GetPlayerCharacter` 0))))
    (bind _returnvalue_2 (message `/Game/BackroomsHole/Blueprint/HUD/Yndrr_BPI_HUD_Interface.GetDialogueInHUD` _returnvalue))
    (if (not (`Widget.IsVisible` _returnvalue_2))
      (bind _returnvalue_3 (message `/Game/BackroomsHole/Blueprint/HUD/Yndrr_BPI_HUD_Interface.GetSaveMenuInHUD` _returnvalue))
      (if (not (`Widget.IsVisible` _returnvalue_3))
        (bind _returnvalue_4 (message `/Game/BackroomsHole/Blueprint/HUD/Yndrr_BPI_HUD_Interface.GetActorViewerInHUD` _returnvalue))
        (if (not (`Widget.IsVisible` _returnvalue_4))
          (bind _returnvalue_5 (message `/Game/BackroomsHole/Blueprint/HUD/Yndrr_BPI_HUD_Interface.GetInventoryInHUD` _returnvalue))
          (if (`Widget.IsVisible` _returnvalue_5)
            _
            (else
              (return true)))))))
  (return false))