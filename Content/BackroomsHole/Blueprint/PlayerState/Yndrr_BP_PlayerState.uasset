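; Player state Blueprint that serves as an access point for player input mode and several gameplay components.
; Input mode set, get, undo and undo-validity calls are forwarded to an InputModeComponent.
; Getters expose the save game, ability system manager and zoom event components, while the camera shake getter returns nothing.
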(event `/Game/LelouFW/Blueprint/PlayerState/LelouFW_BPI_PlayerState_Interface.SetPlayerInputMode`
  (params (Game :type Boolean) (UI :type Boolean) (InWidgetToFocus :type "Widget Object Reference"))
  (`/Game/LelouFW/Blueprint/InputMode/LelouFW_BP_InputMode_ActorComponent.SetInputMode` (`self.InputModeComponent`) Game UI InWidgetToFocus false))

(event `self.ReceiveBeginPlay`
  (`parent.ReceiveBeginPlay`))

(event `/Game/LelouFW/Blueprint/PlayerState/LelouFW_BPI_PlayerState_Interface.UndoPlayerInputMode`
  (`/Game/LelouFW/Blueprint/InputMode/LelouFW_BP_InputMode_ActorComponent.Undo` (`self.InputModeComponent`)))

(fn `GetAbilitySystemManagerComponent`
  (returns (ReturnValue :type "/Game/BackroomsHole/Blueprint/AbilitySystem/Yndrr_BP_AbilitySystem_Manager_ActorComponent Object Reference"))
  (return (`self.AbilitySystemManagerComponent`)))

(fn `GetCameraShakeComponent`
  (returns (ReturnValue :type "/Game/BackroomsHole/Blueprint/Camera/CameraShake/Yndrr_BP_CameraShake_ActorComponent Object Reference"))
  (return null))

(fn `GetPlayerInputMode`
  (returns (Game :type Boolean) (UI :type Boolean) (WidgetToFocus :type "Widget Object Reference"))
  (bind (_game _ui _widgettofocus) (`/Game/LelouFW/Blueprint/InputMode/LelouFW_BP_InputMode_ActorComponent.GetInputMode` (`self.InputModeComponent`)))
  (return _game _ui _widgettofocus))

(fn `GetSaveGameComponent`
  (returns (ReturnValue :type "/Game/LelouFW/Blueprint/SaveGame/LelouFW_BP_SaveGame_ActorComponent Object Reference"))
  (return (`self.GameplaySaveGameComponent`)))

(fn `GetZoomEventComponent`
  (returns (ReturnValue :type "/Game/LelouFW/Blueprint/ZoomEvent/LelouFW_BP_ZoomEvent_ActorComponent Object Reference"))
  (return (`self.ZoomEventComponent`)))

(fn `UserConstructionScript`
  (`parent.UserConstructionScript`))

(fn `ValidUndoPlayerInputMode`
  (returns (ReturnValue :type Boolean))
  (return (`/Game/LelouFW/Blueprint/InputMode/LelouFW_BP_InputMode_ActorComponent.ValidUndo` (`self.InputModeComponent`))))