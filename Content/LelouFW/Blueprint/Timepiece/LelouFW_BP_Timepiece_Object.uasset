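; Clock logic object that keeps a timespan, starting from a given time or Now, and broadcasts each change through OnTimeChanged.
; A looping, gated timer advances the time by its interval, or rewinds it when Reverse is set.
; Paralysis or Speedy switches playback to a 60 Hz broken-clock timer.
; Paralysis broadcasts randomized offsets to mimic a twitching second hand without altering stored time, while Speedy races time by about a minute per tick.
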(event `/Game/LelouFW/Blueprint/Timepiece/LelouFW_BPI_Timepiece_Interface.StartTimepiece`
  (params (StartTime :type "Timespan Structure") (IntervalSecond :type "Float (double-precision)"))
  (`self.Start` StartTime IntervalSecond))

(event `Start`
  (params (StartTime :type "Timespan Structure") (IntervalSecond :type "Float (single-precision)" :default 0.0))
  (if (not (stale `SetWorking` NewWorking))
    (`|ExecutionSequence`
      (:`then_0`
        (`self.SetStartTime` StartTime))
      (:`then_1`
        (`self.SetWorking` true))
      (:`then_2`
        (`self.Play` IntervalSecond)))))

(event `SetTimepieceInterval`
  (params (TimepieceInterval :type "Float (single-precision)"))
  (if (and (!= (stale `SetTimepieceInterval` _output_get) TimepieceInterval) (< 0.0 TimepieceInterval))
    (`|ExecutionSequence`
      (:`then_0`
        (bind _output_get (set `self.TimepieceInterval` TimepieceInterval)))
      (:`then_1`
        (`/Engine/EditorBlueprintResources/StandardMacros.Gate` true :!label _label
          (:`Exit`
            (`|ExecutionSequence`
              (:`then_0`
                (`KismetSystemLibrary.K2_ClearTimer` null "TimepieceTimer" :!label _label_2))
              (:`then_1`
                (`KismetSystemLibrary.K2_SetTimer` null "TimepieceTimer" _output_get true :!label _label_3)))))))))

(event `/Game/LelouFW/Blueprint/Timepiece/LelouFW_BPI_Timepiece_Interface.SetTimepieceStartTime`
  (params (StartTime :type "Timespan Structure"))
  (`self.SetStartTime` StartTime))

(event `SetWorking`
  (params (NewWorking :type Boolean)))

(event `PlayTimepiece`
  (params (IntervalSecond :type "Float (single-precision)" :default 1.0))
  (`|ExecutionSequence`
    (:`then_0`
      (`self.SetTimepieceInterval` IntervalSecond))
    (:`then_1`
      (`self.TimepieceTimer`))
    (:`then_2`
      (goto _label_3))
    (:`then_3`
      (goto _label :!via `Open`))))

(event `/Game/LelouFW/Blueprint/Timepiece/LelouFW_BPI_Timepiece_Interface.StopTimepiece`
  (`self.Stop`))

(event `SetReverse`
  (params (NewReverse :type Boolean))
  (set `self.Reverse` NewReverse))

(event `StopTimepieceTimer`
  (`|ExecutionSequence`
    (:`then_0`
      (goto _label_2))
    (:`then_1`
      (goto _label :!via `Close`))))

(event `/Game/LelouFW/Blueprint/Timepiece/LelouFW_BPI_Timepiece_Interface.SetParalysisAtTimepiece`
  (params (Paralysis :type Boolean))
  (`self.SetParalysis` Paralysis))

(event `SetCurrentTime`
  (params (CurrentTime :type "Timespan Structure"))
  (bind _output_get (set `self.CurrentTime` CurrentTime))
  (`self.CallTimeChangedEventDispatcher` _output_get))

(event `/Game/LelouFW/Blueprint/Timepiece/LelouFW_BPI_Timepiece_Interface.SetReverseAtTimepiece`
  (params (Reverce :type Boolean))
  (`self.SetReverse` Reverce))

(event `SetStartTime`
  (params (StartTime :type "Timespan Structure"))
  (if (!= StartTime (`KismetMathLibrary.TimespanZeroValue`))
    (`self.SetCurrentTime` StartTime)
    (else
      (bind _returnvalue (`self.Get Timespan by Date Time` (`KismetMathLibrary.Now`)))
      (`self.SetCurrentTime` _returnvalue))))

(event `TimepieceTimer`
  (if (and (stale `SetWorking` NewWorking) (not (`self.Is Broken`)))
    (`self.CalculationCurrentTime` (`KismetMathLibrary.MakeTimespan` 0 0 0 0 (`KismetMathLibrary.FTrunc` (* (stale `SetTimepieceInterval` _output_get) 1000.0))))))

(event `/Game/LelouFW/Blueprint/Timepiece/LelouFW_BPI_Timepiece_Interface.SetSpeedyAtTimepiece`
  (params (Speedy :type Boolean))
  (`self.SetSpeedy` Speedy))

(event `CalculationCurrentTime`
  (params (Timespan :type "Timespan Structure"))
  (bind _returnvalue (`self.GetCurrentTime`))
  (`self.SetCurrentTime` (`self.CalcTimespan` _returnvalue Timespan)))

(event `PlayBreak`
  ;[1 1 1] Break
  (if (`self.Is Broken`)
    (`|ExecutionSequence`
      (:`then_0`
        (`/Engine/EditorBlueprintResources/StandardMacros.DoOnce` false
          (:`Completed`
            (`KismetSystemLibrary.K2_SetTimerDelegate` (delegate `BreakTimer`) (/ 1.0 (`KismetMathLibrary.Conv_IntToDouble` 60)) true))))
      (:`then_1`
        (goto _label_4 :!via `Open`)))))

(event `CallTimeChangedEventDispatcher`
  (params (Timespan :type "Timespan Structure"))
  (`self.OnTimeChanged` Timespan))

(event `BreakTimer`
  ;[1 1 1] Break
  (`/Engine/EditorBlueprintResources/StandardMacros.Gate` false :!label _label_4
    (:`Exit`
      (if (stale `SetWorking` NewWorking)
        (if (stale `SetParalysis` _output_get)
          (`self.ParalysisTimer`)
          (elif (stale `SetSpeedy` _output_get)
            (`self.SpeedyTimer`)))))))

(event `Stop`
  (`self.StopTimers`)
  (`self.SetWorking` false))

(event `StopBreak`
  ;[1 1 1] Break
  (`|ExecutionSequence`
    (:`then_0`
      (goto _label_5 :!via `Reset`))
    (:`then_1`
      (goto _label_4 :!via `Close`))))

(event `StopTimers`
  (`|ExecutionSequence`
    (:`then_0`
      (`self.StopTimepieceTimer`))
    (:`then_1`
      (`self.StopBreak`))))

(event `SetParalysis`
  (params (NewParalysis :type Boolean))
  ;[1 1 1] Break
  (bind _output_get (set `self.Paralysis` NewParalysis))
  (`self.Play` (stale `Start` IntervalSecond)))

(event `SetSpeedy`
  (params (NewSpeedy :type Boolean))
  ;[1 1 1] Break
  (bind _output_get (set `self.Speedy` NewSpeedy))
  (`self.Play` (stale `Start` IntervalSecond)))

(event `Play`
  (params (IntervalSecond :type "Float (single-precision)"))
  (if (`self.Is Broken`)
    (`self.PlayBreak`)
    (elif (< 0.0 IntervalSecond)
      (`self.PlayTimepiece` IntervalSecond)
      (else
        (`self.PlayTimepiece` (`self.DefaultIntervalSecond`))))))

(event `ParalysisTimer`
  ;[1 1 1] Break
  ;;[1 1 1] Paralysis（秒針が痙攣する壊れた表現）
  (`|ExecutionSequence`
    (:`then_0`
      (`/Engine/EditorBlueprintResources/StandardMacros.DoOnce` false :!label _label_5
        (:`Completed`
          (`|ExecutionSequence`
            (:`then_0`
              (bind _returnvalue (`self.GetCurrentTime`)))
            (:`then_1`
              (goto _label_6 :!via `Reset`))))))
    (:`then_1`
      (bind _counter (`/Engine/EditorBlueprintResources/StandardMacros.Do N` 60 :!label _label_6)
        (:`Exit`
          (if (<= _counter (* (`KismetMathLibrary.Conv_IntToDouble` 60) 0.8))
            (`self.CallTimeChangedEventDispatcher` (`self.CalcTimespan` _returnvalue (`KismetMathLibrary.MakeTimespan` 0 0 0 0 (`KismetMathLibrary.FTrunc` (`KismetMathLibrary.Lerp` 600.0 700.0 (`KismetMathLibrary.RandomFloat`))))))
            (else
              (`|ExecutionSequence`
                (:`then_0`
                  (`/Engine/EditorBlueprintResources/StandardMacros.DoOnce` false :!label _label_7
                    (:`Completed`
                      (`self.CallTimeChangedEventDispatcher` _returnvalue))))
                (:`then_1`
                  (if (<= 60 _counter)
                    (`|ExecutionSequence`
                      (:`then_0`
                        (goto _label_7 :!via `Reset`))
                      (:`then_1`
                        (goto _label_6 :!via `Reset`)))))))))))))

(event `SpeedyTimer`
  ;[1 1 1] Break
  ;;[1 1 1] Speedy（壊れた高速回転する表現）
  (`self.CalculationCurrentTime` (`KismetMathLibrary.MakeTimespan` 0 0 1 0 500)))

(fn `CalcTimespan`
  (params (Timespan1 :type "Timespan Structure") (Timespan2 :type "Timespan Structure"))
  (returns (ReturnValue :type "Timespan Structure"))
  (if (`self.Reverse`)
    (return (- Timespan1 Timespan2))
    (else
      (return (+ Timespan1 Timespan2)))))

(fn `Get Timespan by Date Time`
  (params (DateTime :type "DateTime Structure"))
  (returns (ReturnValue :type "Timespan Structure"))
  (bind (_year _month _day _hour _minute _second _millisecond) (`KismetMathLibrary.BreakDateTime` DateTime))
  (return (`KismetMathLibrary.MakeTimespan` _day _hour _minute _second _millisecond)))

(fn `GetCurrentTime`
  (returns (ReturnValue :type "Timespan Structure"))
  (return (`self.CurrentTime`)))

(fn `Is Broken`
  (returns (ReturnValue :type Boolean))
  (return (or (`self.Paralysis`) (`self.Speedy`))))