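; Actor component that plays, tracks and controls force feedback components, applying a shared intensity multiplier and stopping them all on request.
; Played components join a unique list, which arms pause monitoring through a one-time setup and a gate.
; A pause-change binding and a gated Tick check zero the intensity while the game is paused, then restore the stored multiplier.
; Ticking while paused is enabled only when WatchGamePaused is set.
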(event `/Game/LelouFW/Blueprint/ForceFeedback/LelouFW_BPI_ForceFeedback_Interface.PlayForceFeedback`
  (params (ForceFeedbackComponent :type "ForceFeedbackComponent Object Reference") (StartTime :type "Float (double-precision)"))
  (`self.Play` ForceFeedbackComponent StartTime))

(event `SetupGamePaused`
  ;[1 1 1] GamePaused
  (`/Engine/EditorBlueprintResources/StandardMacros.DoOnce` false
    (:`Completed`
      (`|ExecutionSequence`
        (:`then_0`
          (if (`self.WatchGamePaused`)
            (`self.SetTickableWhenPaused` true)))
        (:`then_1`
          (add `self.OnGamePausedChanged` (delegate `BindGamePaused`)))))))

(event `self.ReceiveTick`
  (params (DeltaSeconds :type "Float (single-precision)"))
  (`self.WatchGamePausedTimer`))

(event `BindGamePaused` :!signature `self.OnGamePausedChanged`
  (params (GamePaused :type Boolean))
  ;[1 1 1] GamePaused
  (bind _returnvalue (`self.GetForceFeedbacks`))
  (if GamePaused
    (`ForceFeedbackComponent.SetIntensityMultiplier` _returnvalue 0.0)
    (else
      (bind _returnvalue_2 (`self.GetIntensityMultiplier`))
      (`ForceFeedbackComponent.SetIntensityMultiplier` _returnvalue _returnvalue_2))))

(event `Play`
  (params (ForceFeedback :type "ForceFeedbackComponent Object Reference") (StartTime :type "Float (single-precision)"))
  (`/Engine/EditorBlueprintResources/StandardMacros.IsValid` ForceFeedback
    (:`Is Valid`
      (`|ExecutionSequence`
        (:`then_0`
          (`self.AddForceFeedback` ForceFeedback))
        (:`then_1`
          (bind _returnvalue (`self.GetIntensityMultiplier`))
          (`self.SetIntensityMultiplier` _returnvalue))
        (:`then_2`
          (`ForceFeedbackComponent.Play` ForceFeedback StartTime))))))

(event `WatchGamePausedTimer`
  (bind _returnvalue (`GameplayStatics.IsGamePaused`))
  ;[1 1 1] GamePaused
  (`/Engine/EditorBlueprintResources/StandardMacros.Gate` true :!label _label
    (:`Exit`
      (if (!= (stale `BindGamePaused` GamePaused) _returnvalue)
        (`self.BindGamePaused` _returnvalue)))))

(event `StopStandbyGamePaused`
  ;[1 1 1] GamePaused
  (goto _label :!via `Close`))

(event `Stop`
  (bind _returnvalue (`self.GetForceFeedbacks`))
  (`ForceFeedbackComponent.Stop` _returnvalue))

(event `StandbyGamePaused`
  ;[1 1 1] GamePaused
  (`|ExecutionSequence`
    (:`then_0`
      (`self.SetupGamePaused`))
    (:`then_1`
      (goto _label :!via `Open`))))

(event `SetIntensityMultiplier`
  (params (NewIntensityMultiplier :type "Float (single-precision)" :default 1.0))
  (bind _output_get (set `self.IntensityMultiplier` NewIntensityMultiplier))
  (bind _returnvalue (`self.GetForceFeedbacks`))
  (`ForceFeedbackComponent.SetIntensityMultiplier` _returnvalue _output_get))

(event `AddForceFeedback`
  (params (ForceFeedback :type "ForceFeedbackComponent Object Reference (by ref)"))
  (bind _returnvalue (`KismetArrayLibrary.Array_AddUnique` (`self.ForceFeedbacks`) ForceFeedback))
  (if (<= 0 _returnvalue)
    (`self.StandbyGamePaused`)))

(fn `GetForceFeedbacks`
  (returns (ReturnValue :type "Array of ForceFeedbackComponent Object Reference"))
  (return (`self.ForceFeedbacks`)))

(fn `GetIntensityMultiplier`
  (returns (ReturnValue :type "Float (double-precision)"))
  (return (`self.IntensityMultiplier`)))