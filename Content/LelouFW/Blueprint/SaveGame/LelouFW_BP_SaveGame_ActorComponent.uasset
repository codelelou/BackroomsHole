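; Actor component that saves and loads save-game slots asynchronously, firing start and completion dispatchers for each operation.
; Save and existence checks fall back to the default slot name when none is given, while load uses the name as passed.
; Gameplay saves write a valid object as is, otherwise take the GameInstance's, stamped with time and player transform.
; Helper functions expose slot names, including numbered custom slots.
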(event `/Game/LelouFW/Blueprint/SaveGame/LelouFW_BPI_SaveGame_ActorComponent_Interface.SaveGame`
  (params (SaveGameObject :type "SaveGame Object Reference") (SlotName :type String) (UserIndex :type Integer))
  (`self.Save` SaveGameObject SlotName UserIndex))

(event `Load`
  (params (SlotName :type String) (UserIndex :type Integer))
  ;[1 1 1] LoadGame
  (bind (_savegame _bsuccess) (`AsyncActionHandleSaveGame.AsyncLoadGameFromSlot` SlotName UserIndex)
    (:`then`
      (`self.BindStartLoadGame` SlotName UserIndex))
    (:`Completed`
      (`self.BindCompletedLoadGame` _savegame _bsuccess SlotName UserIndex))))

(event `/Game/LelouFW/Blueprint/SaveGame/LelouFW_BPI_SaveGame_ActorComponent_Interface.SaveGameplaySaveGame`
  (params (SaveGame :type "SaveGame Object Reference") (SlotName :type String) (UserIndex :type Integer))
  (`self.SaveGameplay` SaveGame SlotName UserIndex))

(event `BindStartLoadGame`
  (params (SlotName :type String) (UserIndex :type Integer))
  ;[1 1 1] LoadGame
  (`self.OnStartLoadGame` SlotName UserIndex))

(event `/Game/LelouFW/Blueprint/SaveGame/LelouFW_BPI_SaveGame_ActorComponent_Interface.LoadGame`
  (params (SlotName :type String) (UserIndex :type Integer))
  (`self.Load` SlotName UserIndex))

(event `Save`
  (params (SaveGameObject :type "SaveGame Object Reference") (SlotName :type String) (UserIndex :type Integer))
  ;[1 1 1] Save
  (bind _returnvalue (`self.FilterSlotName` SlotName))
  (bind (_savegame _bsuccess) (`AsyncActionHandleSaveGame.AsyncSaveGameToSlot` SaveGameObject _returnvalue UserIndex)
    (:`then`
      (`self.CallStartSaveGameEventDispatcher` SaveGameObject _returnvalue UserIndex))
    (:`Completed`
      (`self.CallCompletedSaveGameEventDispatcher` _savegame _bsuccess _returnvalue UserIndex))))

(event `BindCompletedLoadGame`
  (params (SaveGame :type "SaveGame Object Reference") (Success :type Boolean) (SlotName :type String) (UserIndex :type Integer))
  ;[1 1 1] LoadGame
  (`self.OnCompletedLoadGame` SaveGame Success SlotName UserIndex))

(event `CallStartSaveGameEventDispatcher`
  (params (SaveGameObject :type "SaveGame Object Reference") (SlotName :type String) (UserIndex :type Integer))
  ;[1 1 1] Save
  (`self.OnStartSaveGame` SaveGameObject SlotName UserIndex))

(event `CallCompletedSaveGameEventDispatcher`
  (params (SaveGameObject :type "SaveGame Object Reference") (Success :type Boolean) (SlotName :type String) (UserIndex :type Integer))
  ;[1 1 1] Save
  (`self.OnCompletedSaveGame` SaveGameObject Success SlotName UserIndex))

(event `SaveGameplay`
  (params (SaveGame :type "SaveGame Object Reference") (SlotName :type String) (UserIndex :type Integer))
  (`/Engine/EditorBlueprintResources/StandardMacros.IsValid` SaveGame
    (:`Is Valid`
      (`self.Save` SaveGame SlotName UserIndex))
    (:`Is Not Valid`
      (bind _returnvalue (`self.ConvertGameplayForSave` null))
      (`self.Save` _returnvalue SlotName UserIndex))))

(fn `ConvertGameplayForSave`
  (params (SaveGame :type "SaveGame Object Reference"))
  (returns (ReturnValue :type "SaveGame Object Reference"))
  (locals (SGame :type "SaveGame Object Reference"))
  (bind _output_get (set `local.SGame` SaveGame))
  (`|ExecutionSequence`
    (:`then_0`
      (`/Engine/EditorBlueprintResources/StandardMacros.IsValid` _output_get
        (:`Is Not Valid`
          (bind _returnvalue (`self.GetGameplay`))
          (set `local.SGame` _returnvalue))))
    (:`then_1`
      (message `/Game/LelouFW/Blueprint/SaveGame/Gameplay/LelouFW_BPI_SaveGame_Gameplay_Interface.SetTimestampAtSaveGame` _output_get (`KismetMathLibrary.Now`)))
    (:`then_2`
      (message `/Game/LelouFW/Blueprint/SaveGame/Gameplay/LelouFW_BPI_SaveGame_Gameplay_Interface.SetPlayerTransformByPlayerAtSaveGame` _output_get (`GameplayStatics.GetPlayerCharacter` 0) (`GameplayStatics.GetPlayerController` 0)))
    (:`then_3`
      (return _output_get))))

(fn `ConvertGameplaySaveGameForSave`
  (params (SaveGame :type "SaveGame Object Reference"))
  (returns (ReturnValue :type "SaveGame Object Reference"))
  (bind _returnvalue (`self.ConvertGameplayForSave` SaveGame))
  (return _returnvalue))

(fn `DoesSaveGameExist`
  (params (SlotName :type String) (UserIndex :type Integer))
  (returns (ReturnValue :type Boolean))
  (bind _returnvalue (`self.FilterSlotName` SlotName))
  (bind _returnvalue_2 (`GameplayStatics.DoesSaveGameExist` _returnvalue UserIndex))
  (return _returnvalue_2))

(fn `FilterSlotName`
  (params (SlotName :type String))
  (returns (ReturnValue :type String))
  (if (`KismetStringLibrary.IsEmpty` SlotName)
    (return (`self.GetSlotName`))
    (else
      (return SlotName))))

(fn `GetCustomSlotNames`
  (returns (CustomSlotNames :type "Array of String"))
  (locals (CSNames :type "Array of String"))
  (bind _csnames (`local.CSNames`))
  (for _index (range 1 (+ (`self.Customs`) 1))
    (`KismetArrayLibrary.Array_AddUnique` _csnames (`KismetTextLibrary.Conv_TextToString` (`|FormatText` "{Prefix}_{Number}" (`self.SlotName`) (`KismetTextLibrary.Conv_IntToText` _index false false 3)))))
  (return _csnames))

(fn `GetGameplay`
  (returns (ReturnValue :type "SaveGame Object Reference"))
  (bind _returnvalue (message `/Game/LelouFW/Blueprint/GameInstance/LelouFW_BPI_GameInstance_Gameplay_Interface.GetGameplaySaveGame` (`GameplayStatics.GetGameInstance`)))
  (return _returnvalue))

(fn `GetGameplayCustomSlotNames`
  (returns (ReturnValue :type "Array of String"))
  (bind _customslotnames (`self.GetCustomSlotNames`))
  (return _customslotnames))

(fn `GetSaveGameSlotName`
  (returns (ReturnValue :type String))
  (return (`self.GetSlotName`)))

(fn `GetSlotName`
  (returns (SlotName :type String))
  (return (`self.SlotName`)))

(fn `IsSaveGame`
  (params (SlotName :type String) (UserIndex :type Integer))
  (returns (ReturnValue :type Boolean))
  (bind _returnvalue (`self.DoesSaveGameExist` SlotName UserIndex))
  (return _returnvalue))