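; Base actor-viewer model that presents a world actor in front of the player camera for inspection.
; Show saves the actor's transforms and collision state, then after short timer delays places it facing the camera with collision off.
; Control-flag-gated inputs rotate it, scale it within half to double the initial size, and move it tick by tick within a limit.
; Hide cancels the timers, restores transforms and collision, and fires the visibility dispatcher.
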(event `/Game/LelouFW/Blueprint/ActorViewer/LelouFW_BPI_ActorViewer_Model_Interface.ShowActorViewer`
  (params (Item :type "Actor Object Reference"))
  (`self.Show` Item))

(event `ShowItem`
  (`|ExecutionSequence`
    (:`then_0`
      (`self.UpdateCollision` true))
    (:`then_1`
      (`self.SetupBeginShowItem`))
    (:`then_2`
      (`self.CallVisibilityChangedEventDispatcher` true))
    (:`then_3`
      (`self.SetItemControl` true))))

(event `CallVisibilityChangedEventDispatcher`
  (params (Visibility :type Boolean))
  (bind _actor (`self.GetItem`))
  (`self.OnActorVIewerVisibilityChanged` Visibility _actor))

(event `AddRotateItem`
  (params (Value :type "Rotator Structure"))
  ;[1 1 1] Item Rotate
  (if (`self.AvailableRotateControl`)
    (bind (_actor _itemscene) (`self.GetItem`))
    (`SceneComponent.K2_SetRelativeRotation` _itemscene (`KismetMathLibrary.ComposeRotators` (`SceneComponent.RelativeRotation` _itemscene) Value) false false)))

(event `SetItemControl`
  (params (NewAvailable :type Boolean))
  (set `self.ItemControl` NewAvailable))

(event `/Game/LelouFW/Blueprint/ActorViewer/LelouFW_BPI_ActorViewer_Model_Interface.HideActorViewer`
  (`self.Hide`))

(event `HideItem`
  (`|ExecutionSequence`
    (:`then_0`
      (`self.SetItemControl` false))
    (:`then_1`
      (`self.ResetActorProperty`))
    (:`then_2`
      (`self.UpdateCollision` false))
    (:`then_3`
      (`self.CallVisibilityChangedEventDispatcher` false))))

(event `ResetActorProperty`
  ;[1 1 1] Actor復元用
  (bind (_actor _itemscene) (`self.GetItem`))
  (`|ExecutionSequence`
    (:`then_0`
      (`SceneComponent.K2_SetWorldTransform` _itemscene (stale `BackupItemProperty` SceneWorldTransform) false false))
    (:`then_1`
      (`SceneComponent.K2_SetRelativeTransform` _itemscene (stale `BackupItemProperty` SceneRelativeTransform) false false))
    (:`then_2`
      (`self.K2_SetActorTransform` _actor (stale `BackupItemProperty` ActorWorldTransform) false false))))

(event `AddItemRotationFromVector`
  (params (Value :type "Vector Structure"))
  ;[1 1 1] Item Rotate
  (if (!= Value (0.0 0.0 0.0) :`ErrorTolerance` 0.15)
    (`self.AddRotateItem` (`KismetMathLibrary.MakeRotator` 0.0 (* (.y Value) (`KismetMathLibrary.Abs` -20.0)) (* (.x Value) -20.0)))))

(event `/Game/LelouFW/Blueprint/ActorViewer/LelouFW_BPI_ActorViewer_Model_Interface.SetActorViewerItemTransform`
  (params (Transform :type "Transform Structure"))
  (`self.SetItemTransform` Transform))

(event `BackupItemProperty`
  (params (ActorWorldTransform :type "Transform Structure") (SceneWorldTransform :type "Transform Structure") (SceneRelativeTransform :type "Transform Structure") (EnableCollision :type Boolean))
  ;[1 1 1] Actor復元用
)

(event `AddRotateItemVertical`
  (params (Value :type "Float (double-precision)"))
  ;[1 1 1] Item Rotate
  (if (not (`KismetMathLibrary.NearlyEqual_FloatFloat` Value 0.0 0.15))
    (`self.AddRotateItem` (`KismetMathLibrary.MakeRotator` 0.0 (* Value -20.0)))))

(event `/Game/LelouFW/Blueprint/ActorViewer/LelouFW_BPI_ActorViewer_Model_Interface.AddScaleAtActorViewerItem`
  (params (Value :type "Float (double-precision)"))
  (`self.AddScaleItem` Value))

(event `AddRotateItemHorizontal`
  (params (Value :type "Float (double-precision)"))
  ;[1 1 1] Item Rotate
  (if (not (`KismetMathLibrary.NearlyEqual_FloatFloat` Value 0.0 0.15))
    (`self.AddRotateItem` (`KismetMathLibrary.MakeRotator` 0.0 0.0 (* Value -20.0)))))

(event `/Game/LelouFW/Blueprint/ActorViewer/LelouFW_BPI_ActorViewer_Model_Interface.AddRotateHorizontalAtActorViewerItem`
  (params (Value :type "Float (double-precision)"))
  (`self.AddRotateItemHorizontal` Value))

(event `SetItemScene`
  (params (ItemScene :type "SceneComponent Object Reference"))
  (bind _output_get (set `self.ItemScene` ItemScene))
  (`self.BackupItemProperty` (`self.GetTransform` (stale `SetItem` _output_get)) (`SceneComponent.K2_GetComponentToWorld` _output_get) (`SceneComponent.GetRelativeTransform` _output_get) (`self.GetActorEnableCollision` (stale `SetItem` _output_get))))

(event `/Game/LelouFW/Blueprint/ActorViewer/LelouFW_BPI_ActorViewer_Model_Interface.AddRotateVerticalAtActorViewerItem`
  (params (Value :type "Float (double-precision)"))
  (`self.AddRotateItemVertical` Value))

(event `UpdateCollision`
  (params (IsShow :type Boolean))
  ;[1 1 1] Item Collision
  ; Itemが動く時にCollisionがCharacterに干渉しないようにする
  (if (stale `BackupItemProperty` EnableCollision)
    (bind _actor (`self.GetItem`))
    (`self.SetActorEnableCollision` _actor (not IsShow))))

(event `AddScaleItem`
  (params (Value :type "Float (double-precision)"))
  ;[1 1 1] Item Scale
  (if (`self.AvailableScaleControl`)
    (bind (_actor _itemscene) (`self.GetItem`))
    (if (not (`KismetMathLibrary.NearlyEqual_FloatFloat` 0.0 Value 0.001))
      (bind _returnvalue (`KismetMathLibrary.Vector_GetAbs` (+ (`SceneComponent.K2_GetComponentScale` _itemscene) Value)))
      (bind (_minscale _maxscale) (`self.GetScaleRange` (.scale (stale `SetItemTransform` Transform))))
      (if (`KismetMathLibrary.InRange_FloatFloat` (`KismetMathLibrary.Vector_GetAbsMin` _returnvalue) _minscale _maxscale)
        (`SceneComponent.SetWorldScale3D` _itemscene _returnvalue) ; RootComponent対応でWorldScale
      ))))

(event `/Game/LelouFW/Blueprint/ActorViewer/LelouFW_BPI_ActorViewer_Model_Interface.AddLocationHorizontalAtActorViewerItem`
  (params (Value :type "Float (double-precision)"))
  (`self.AddLocationItemHorizontal` Value))

(event `SetItem`
  (params (Item :type "Actor Object Reference"))
  (`/Engine/EditorBlueprintResources/StandardMacros.IsValid` Item
    (:`Is Valid`
      (bind _output_get (set `self.ItemActor` Item))
      (`self.SetItemScene` (`Actor.RootComponent` _output_get)))))

(event `SetupCamera`
  ;[1 1 1] Camera
  (`/Engine/EditorBlueprintResources/StandardMacros.DoOnce` false
    (:`Completed`
      (`/Engine/EditorBlueprintResources/StandardMacros.IsValid` (stale `SetCamera` _output_get)
        (:`Is Not Valid`
          (`self.SetCamera` (`Actor.RootComponent` (`GameplayStatics.GetPlayerCameraManager` 0))))))))

(event `/Game/LelouFW/Blueprint/ActorViewer/LelouFW_BPI_ActorViewer_Model_Interface.AddLocationVerticalAtActorViewerItem`
  (params (Value :type "Float (double-precision)"))
  (`self.AddLocationItemVertical` Value))

(event `SetCamera`
  (params (Camera :type "SceneComponent Object Reference"))
  ;[1 1 1] Camera
  (bind _output_get (set `self.Camera` Camera)))

(event `Show`
  (params (Item :type "Actor Object Reference"))
  (`/Engine/EditorBlueprintResources/StandardMacros.DoOnce` false :!label _label
    (:`Completed`
      (`|ExecutionSequence`
        (:`then_0`
          (`self.SetItem` Item))
        (:`then_1`
          (bind _returnvalue (`KismetSystemLibrary.K2_SetTimerDelegate` (delegate `ShowDelayA`) 0.1)))))))

(event `/Game/LelouFW/Blueprint/ActorViewer/LelouFW_BPI_ActorViewer_Model_Interface.ResetActorViewerItem`
  (`self.ResetItem`))

(event `SetItemTransform`
  (params (Transform :type "Transform Structure")))

(event `ShowDelayA`
  ;[1 0 0] TODO: キャラクター移動直後などのカメラ位置対応の暫定遅延処理
  (`|ExecutionSequence`
    (:`then_0`
      (bind _actor (`self.GetItem`))
      (`self.SetActorHiddenInGame` _actor false) ; TODO: インベントリ経由で表示する用（非表示はCustomActorで実施）
    )
    (:`then_1`
      (`self.ShowItem`))
    (:`then_2`
      (bind _returnvalue (`KismetSystemLibrary.K2_SetTimerDelegate` (delegate `DelayShowB`) 0.4)))))

(event `AddLocationItem`
  ;[1 1 1] Item Location
  (`/Engine/EditorBlueprintResources/StandardMacros.DoOnce` false :!label _label_2
    (:`Completed`
      (bind (_actor _itemscene) (`self.GetItem`))
      (bind _returnvalue (`KismetMathLibrary.GetMaxElement` (.scale (stale `SetItemTransform` Transform))))
      (bind _returnvalue_2 (/ (`KismetMathLibrary.MakeVector` 0.0 (stale `AddLocationItemHorizontal` Value) (stale `AddLocationItemVertical` Value)) _returnvalue))
      (if (and (`self.AvailableMoveControl`) (!= _returnvalue_2 (0.0 0.0 0.0) :`ErrorTolerance` 0.15)) :!label _label_3
        (bind _returnvalue_3 (+ (`SceneComponent.RelativeLocation` _itemscene) _returnvalue_2))
        (bind _returnvalue_4 (/ (`self.MoveLimit`) _returnvalue))
        (if (`KismetMathLibrary.Vector_IsNearlyZero` (`KismetMathLibrary.MakeVector` 0.0 (.y _returnvalue_3) (.z _returnvalue_3)) _returnvalue_4)
          (`|ExecutionSequence`
            (:`then_0`
              (`SceneComponent.K2_SetRelativeLocation` _itemscene _returnvalue_3 false false))
            (:`then_1`
              (`KismetSystemLibrary.DelayUntilNextTick`)
              (goto _label_3)))
          (else
            (`|ExecutionSequence`
              (:`then_0`
                (if (`KismetMathLibrary.NearlyEqual_FloatFloat` (.y _returnvalue_3) 0.0 _returnvalue_4)
                  (if (not (`KismetMathLibrary.NearlyEqual_FloatFloat` (.z _returnvalue_3) 0.0 _returnvalue_4))
                    (`self.AddLocationItemVertical` 0.0 :!label _label_4))
                  (else
                    (`self.AddLocationItemHorizontal` 0.0 :!label _label_5))))
              (:`then_1`
                (goto _label_2 :!via `Reset`)))))
        (else
          (`|ExecutionSequence`
            (:`then_0`
              (goto _label_5))
            (:`then_1`
              (goto _label_4))
            (:`then_2`
              (goto _label_2 :!via `Reset`))))))))

(event `SetupBeginShowItem`
  (bind _returnvalue (`self.GetCamera`))
  (bind _actor (`self.GetItem`))
  (bind _location (.location (`SceneComponent.K2_GetComponentToWorld` _returnvalue)))
  (bind _returnvalue_2 (+ _location (* (`KismetMathLibrary.GetForwardVector` (.rotation (`SceneComponent.K2_GetComponentToWorld` _returnvalue))) (`self.CameraDistance`))))
  (`self.K2_SetActorTransform` _actor (`KismetMathLibrary.MakeTransform` _returnvalue_2 (`KismetMathLibrary.FindLookAtRotation` _returnvalue_2 _location) (.scale (stale `SetItemTransform` Transform))) false false))

(event `DelayShowB`
  ;[1 0 0] TODO: キャラクター移動直後などのカメラ位置対応の暫定遅延処理
  (`self.ShowItem`))

(event `Hide`
  (`|ExecutionSequence`
    (:`then_0`
      (`KismetSystemLibrary.K2_ClearAndInvalidateTimerHandle` (stale `Show` _returnvalue))
      (`KismetSystemLibrary.K2_ClearAndInvalidateTimerHandle` (stale `ShowDelayA` _returnvalue)))
    (:`then_1`
      (`self.HideItem`))
    (:`then_2`
      (goto _label :!via `Reset`))))

(event `AddLocationItemHorizontal`
  (params (Value :type "Float (double-precision)"))
  ;[1 1 1] Item Location
  (`self.AddLocationItem` :!label _label_6))

(event `ResetItem`
  (if (`self.AvailableItemControl`)
    (`self.SetupBeginShowItem`)))

(event `AddLocationItemVertical`
  (params (Value :type "Float (double-precision)"))
  ;[1 1 1] Item Location
  (goto _label_6))

(fn `AvailableItemControl`
  (returns (ReturnValue :type Boolean))
  (return (`self.ItemControl`)))

(fn `AvailableMoveControl`
  (returns (ReturnValue :type Boolean))
  (return (and (`self.AvailableItemControl`) (`self.MoveControl`))))

(fn `AvailableRotateControl`
  (returns (ReturnValue :type Boolean))
  (return (and (`self.AvailableItemControl`) (`self.RotateControl`))))

(fn `AvailableScaleControl`
  (returns (ReturnValue :type Boolean))
  (return (and (`self.AvailableItemControl`) (`self.ScaleControl`))))

(fn `GetActor`
  (returns (ReturnValue :type "Actor Object Reference"))
  (return (`self.ItemActor`)))

(fn `GetActorOnActorViewer`
  (returns (ReturnValue :type "Actor Object Reference"))
  (bind _returnvalue (`self.GetActor`))
  (return _returnvalue))

(fn `GetCamera`
  (returns (ReturnValue :type "SceneComponent Object Reference"))
  (`self.SetupCamera`)
  (return (`self.Camera`)))

(fn `GetItem`
  (returns (Actor :type "Actor Object Reference") (ItemScene :type "SceneComponent Object Reference"))
  (bind _returnvalue (`self.GetActor`))
  (bind _returnvalue_2 (`self.GetItemScene`))
  (return _returnvalue _returnvalue_2))

(fn `GetItemScene`
  (returns (ReturnValue :type "SceneComponent Object Reference"))
  (return (`self.ItemScene`)))

(fn `GetScaleRange`
  (params (ItemScale :type "Vector Structure"))
  (returns (MinScale :type "Float (double-precision)") (MaxScale :type "Float (double-precision)"))
  (locals (Max :type "Float (double-precision)") (Min :type "Float (double-precision)"))
  (bind _returnvalue (`KismetMathLibrary.Vector_GetAbsMin` ItemScale))
  (return (* _returnvalue 0.5) (* _returnvalue 2.0)))

(fn `GetUI`
  (returns (ReturnValue :type "UserWidget Object Reference"))
  (bind _returnvalue (message `/Game/BackroomsHole/Blueprint/HUD/Yndrr_BPI_HUD_Interface.GetActorViewerInHUD` (`PlayerController.GetHUD` (`GameplayStatics.GetPlayerController` 0))))
  (return _returnvalue))

(fn `IsActorViewing`
  (params (Actor :type "Actor Object Reference"))
  (returns (ReturnValue :type Boolean))
  (bind _returnvalue (`/Game/LelouFW/Blueprint/ActorViewer/LelouFW_BPI_ActorViewer_Model_Interface.IsViewing`))
  (if _returnvalue
    (bind _returnvalue_2 (`self.GetUI`))
    (bind _actor (message `/Game/LelouFW/Blueprint/ActorViewer/LelouFW_BPI_WBP_ActorViewer_Interface.GetCurrentActorOnActorViewer` _returnvalue_2))
    (return (== _actor Actor))
    (else
      (return false))))

(fn `IsViewing`
  (returns (ReturnValue :type Boolean))
  (bind _returnvalue (`self.GetUI`))
  (return (`Widget.IsVisible` _returnvalue)))

(fn `UserConstructionScript`)