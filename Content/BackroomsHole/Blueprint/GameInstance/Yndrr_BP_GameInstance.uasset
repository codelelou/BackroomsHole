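; Game instance for BackroomsHole that owns the settings, achievement and gameplay save objects and opens the top menu, gameplay and ending levels.
; On Init it sets a default frame rate limit if none exists, then async-loads settings and achievements, creating and saving defaults when missing.
; Settings drive sound class volumes and LevelHelper actors.
; DoOnce gates block overlapping async saves; gameplay saves stay in memory, created fresh for new games.
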(event `self.ReceiveInit`
  (`parent.ReceiveInit`)
  (`|ExecutionSequence`
    (:`then_0`
      (`self.SetupFrameRate`))
    (:`then_1`
      (`self.LoadSaveGames`))))

(event `/Game/LelouFW/Blueprint/GameInstance/LelouFW_BPI_GameInstance_Level_Interface.ShowTopMenuLevel`
  (`self.OpenTopMenuLevel`))

(event `OpenTopMenuLevel`
  ;[1 1 1] TopMenu
  (`GameplayStatics.OpenLevelBySoftObjectPtr` (`self.TopMenuLevel`)))

(event `LoadSaveGames`
  ;[1 1 1] SaveGame
  (`/Engine/EditorBlueprintResources/StandardMacros.DoOnce` false
    (:`Completed`
      (`|ExecutionSequence`
        (:`then_0`
          (`self.LoadSettings`))
        (:`then_1`
          (`self.LoadAchievement`))))))

(event `/Game/LelouFW/Blueprint/GameInstance/LelouFW_BPI_GameInstance_Level_Interface.ShowEndingLevel`
  (`self.OpenEndingLevel`))

(event `/Game/LelouFW/Blueprint/GameInstance/LelouFW_BPI_GameInstance_Gameplay_Interface.PlayToNewGame`
  (`self.NewGame`))

(event `/Game/LelouFW/Blueprint/GameInstance/LelouFW_BPI_GameInstance_Gameplay_Interface.PlayToContinue`
  (`self.Continue`))

(event `SetupFrameRate`
  ;[1 1 1] FrameRate
  (`/Engine/EditorBlueprintResources/StandardMacros.DoOnce` false
    (:`Completed`
      (bind _returnvalue (`GameUserSettings.GetGameUserSettings`))
      (if (== 0.0 (`GameUserSettings.GetFrameRateLimit` _returnvalue))
        (`GameUserSettings.SetFrameRateLimit` _returnvalue 60.0)
        (`GameUserSettings.ApplySettings` _returnvalue true)))))

(event `OpenEndingLevel`
  ;[1 1 1] Ending
  (`GameplayStatics.OpenLevelBySoftObjectPtr` (`self.EndingLevel`)))

(event `LoadSettings`
  ;[1 1 1] SettingsSaveGame
  (`/Engine/EditorBlueprintResources/StandardMacros.DoOnce` false
    (:`Completed`
      (bind (_savegame _bsuccess) (`AsyncActionHandleSaveGame.AsyncLoadGameFromSlot` (`self.SettingsSlotName`))
        (:`Completed`
          (`|ExecutionSequence`
            (:`then_0`
              (`/Engine/EditorBlueprintResources/StandardMacros.IsValid` _savegame
                (:`Is Valid`
                  (`self.SetSettings` _savegame))
                (:`Is Not Valid`
                  (bind _returnvalue (`self.FactorySettings`))
                  (`|ExecutionSequence`
                    (:`then_0`
                      (`self.SetSettings` _returnvalue))
                    (:`then_1`
                      (`self.SaveSettings`))))))
            (:`then_1`
              (`self.OnLoadCompletedSettingsSaveGame` _savegame _bsuccess))))))))

(event `/Game/LelouFW/Blueprint/GameInstance/LelouFW_BPI_GameInstance_Gameplay_Interface.PlayToGameplay`
  (params (SaveGame :type "SaveGame Object Reference"))
  (`self.Play` SaveGame))

(event `self.SaveSettingsSaveGame`
  (`self.SaveSettings`))

(event `SetSettings`
  (params (SaveGame :type "SaveGame Object Reference"))
  ;[1 1 1] SettingsSaveGame
  (bind _output_get (set `self.SettingsSaveGame` SaveGame))
  (`/Engine/EditorBlueprintResources/StandardMacros.IsValid` _output_get
    (:`Is Valid`
      (`|ExecutionSequence`
        (:`then_0`
          (`self.UpdateSoundClasses`))
        (:`then_1`
          (`self.UpdateLevelHelper`))))))

(event `self.ResetSettingsSaveGame`
  (`self.ResetSettings`))

(event `UpdateLevelHelper`
  (bind _returnvalue (`self.GetSettings`))
  (bind _returnvalue_2 (`self.Find Level Helpers`))
  (message `/Game/LelouFW/Blueprint/Actor/LevelHelper/LelouFW_BPI_Actor_LevelHelper_Interface.UpdateLevelHelperActorBySaveGame` _returnvalue_2 _returnvalue))

(event `OpenMainGameLevel`
  ;[1 1 1] Main Game (Gameplay)
  (`GameplayStatics.OpenLevelBySoftObjectPtr` (`self.GameplayLevel`)))

(event `/Game/LelouFW/Blueprint/GameInstance/LelouFW_BPI_GameInstance_Gameplay_Achievement_Interface.AddGameplayTagToAchievement`
  (params (GameplayTag :type "GameplayTag Structure"))
  (`self.AddAchievement` GameplayTag))

(event `Play`
  (params (GameplaySaveGame :type "SaveGame Object Reference"))
  ;[1 1 1] Main Game (Gameplay)
  (`self.SetGameplaySaveGame` GameplaySaveGame)
  (`self.OpenMainGameLevel`))

(event `SaveSettings`
  ;[1 1 1] SettingsSaveGame
  (`/Engine/EditorBlueprintResources/StandardMacros.DoOnce` false :!label _label
    (:`Completed`
      (bind _returnvalue (`self.GetSettings`))
      (`|ExecutionSequence`
        (:`then_0`
          (`self.OnSaveStartSettingsSaveGame` _returnvalue))
        (:`then_1`
          (bind (_savegame _bsuccess) (`AsyncActionHandleSaveGame.AsyncSaveGameToSlot` _returnvalue (`self.SettingsSlotName`))
            (:`Completed`
              (`|ExecutionSequence`
                (:`then_0`
                  (`self.UpdateLevelHelper`))
                (:`then_1`
                  (`self.OnSaveCompletedSettingsSaveGame` _savegame _bsuccess))
                (:`then_2`
                  (goto _label :!via `Reset`))))))))))

(event `LoadAchievement`
  ;[1 1 1] Achievement
  (`/Engine/EditorBlueprintResources/StandardMacros.DoOnce` false
    (:`Completed`
      (bind (_savegame _bsuccess) (`AsyncActionHandleSaveGame.AsyncLoadGameFromSlot` (`self.AchievementSlotName`))
        (:`Completed`
          (`|ExecutionSequence`
            (:`then_0`
              (`/Engine/EditorBlueprintResources/StandardMacros.IsValid` _savegame
                (:`Is Valid`
                  (`self.SetAchievement` _savegame))
                (:`Is Not Valid`
                  (bind _returnvalue (`self.FactoryAchievement`))
                  (`|ExecutionSequence`
                    (:`then_0`
                      (`self.SetAchievement` _returnvalue))
                    (:`then_1`
                      (`self.SaveAchievement`))))))
            (:`then_1`
              (`self.OnLoadCompletedAchievementSaveGame` _savegame _bsuccess))))))))

(event `NewGame`
  ;[1 1 1] Main Game (Gameplay)
  (bind _returnvalue (`self.FactoryGameplay`))
  (`self.Play` _returnvalue))

(event `Continue`
  ;[1 1 1] Main Game (Gameplay)
  (bind _returnvalue (`self.GetGameplay`))
  (`self.Play` _returnvalue))

(event `ResetSettings`
  ;[1 1 1] SettingsSaveGame
  (bind _returnvalue (`self.FactorySettings`))
  (`|ExecutionSequence`
    (:`then_0`
      (bind _returnvalue_2 (`self.GetSettings`))
      (`|ExecutionSequence`
        (:`then_0`
          (bind _returnvalue_3 (message `/Game/LelouFW/Blueprint/SaveGame/Settings/LelouFW_BPI_SaveGame_Settings_Interface.GetImageQualitySettingsInSaveGame` _returnvalue_2))
          (message `/Game/LelouFW/Blueprint/SaveGame/Settings/LelouFW_BPI_SaveGame_Settings_Interface.SetImageQualitySettingsAtSaveGame` _returnvalue _returnvalue_3))))
    (:`then_1`
      (`self.SetSettings` _returnvalue))
    (:`then_2`
      (`self.SaveSettings`))))

(event `SetAchievement`
  (params (SaveGame :type "SaveGame Object Reference"))
  ;[1 1 1] Achievement
  (set `self.AchievementSaveGame` SaveGame))

(event `SetGameplaySaveGame`
  (params (SaveGame :type "SaveGame Object Reference"))
  ;[1 1 1] Main Game (Gameplay)
  (`/Engine/EditorBlueprintResources/StandardMacros.IsValid` SaveGame
    (:`Is Valid`
      (set `self.GameplaySaveGame` SaveGame))
    (:`Is Not Valid`
      (bind _returnvalue (`self.FactoryGameplay`))
      (set `self.GameplaySaveGame` _returnvalue))))

(event `SaveAchievement`
  ;[1 1 1] Achievement
  (`/Engine/EditorBlueprintResources/StandardMacros.DoOnce` false :!label _label_2
    (:`Completed`
      (bind _returnvalue (`self.GetAchievement`))
      (`|ExecutionSequence`
        (:`then_0`
          (`self.OnSaveStartAchievementSaveGame` _returnvalue))
        (:`then_1`
          (bind (_savegame _bsuccess) (`AsyncActionHandleSaveGame.AsyncSaveGameToSlot` _returnvalue (`self.AchievementSlotName`))
            (:`Completed`
              (`|ExecutionSequence`
                (:`then_0`
                  (`self.OnSaveCompletedAchievementSaveGame` _savegame _bsuccess))
                (:`then_1`
                  (goto _label_2 :!via `Reset`))))))))))

(event `AddAchievement`
  (params (GameplayTag :type "GameplayTag Structure"))
  ;[1 1 1] Achievement
  (bind _returnvalue (`self.GetAchievement`))
  (bind _returnvalue_2 (message `/Game/LelouFW/Blueprint/SaveGame/Achievement/LelouFW_BPI_SaveGame_Achievement_Interface.AddAchievementGameplayTag` _returnvalue GameplayTag))
  (if (<= 0 _returnvalue_2)
    (`self.SaveAchievement`)))

(event `self.UpdateSoundClasses`
  ;[1 1 1] Sound
  (bind _returnvalue (`self.GetSettings`))
  (`|ExecutionSequence`
    (:`then_0`
      (`|ExecutionSequence`
        (:`then_0`
          (bind _returnvalue_2 (message `/Game/LelouFW/Blueprint/SaveGame/Settings/LelouFW_BPI_SaveGame_Settings_Interface.GetBGMSettingsInSaveGame` _returnvalue))
          (`self.SetSoundMixClassOverride` "/Game/BackroomsHole/Sound/Yndrr_SoundClass_BGM.Yndrr_SoundClass_BGM" _returnvalue_2))
        (:`then_1`
          (bind _returnvalue_3 (message `/Game/LelouFW/Blueprint/SaveGame/Settings/LelouFW_BPI_SaveGame_Settings_Interface.GetSoundEffectSettingsInSaveGame` _returnvalue))
          (`self.SetSoundMixClassOverride` "/Game/BackroomsHole/Sound/Yndrr_SoundClass_SoundEffect.Yndrr_SoundClass_SoundEffect" _returnvalue_3))
        (:`then_2`
          (bind _returnvalue_4 (message `/Game/LelouFW/Blueprint/SaveGame/Settings/LelouFW_BPI_SaveGame_Settings_Interface.GetVoiceSettingsInSaveGame` _returnvalue))
          (`self.SetSoundMixClassOverride` "/Game/BackroomsHole/Sound/Yndrr_SoundClass_Voice.Yndrr_SoundClass_Voice" _returnvalue_4))))
    (:`then_1`
      (`GameplayStatics.PushSoundMixModifier` (`self.SoundMix`)))))

(event `SetSoundMixClassOverride`
  (params (InSoundClass :type "SoundClass Object Reference") (Volume :type "Float (single-precision)"))
  ;[1 1 1] Sound
  (`GameplayStatics.SetSoundMixClassOverride` (`self.SoundMix`) InSoundClass Volume))

(fn `FactoryAchievement`
  (returns (ReturnValue :type "SaveGame Object Reference"))
  (bind _returnvalue (`GameplayStatics.CreateSaveGameObject` (`self.AchievementSaveGameClass`)))
  (return _returnvalue))

(fn `FactoryGameplay`
  (returns (ReturnValue :type "/Game/BackroomsHole/Blueprint/SaveGame/Gameplay/Yndrr_BP_SaveGame_Gameplay Object Reference"))
  (bind _returnvalue (`GameplayStatics.CreateSaveGameObject` (`self.GameplaySaveGameClass`)))
  (return _returnvalue))

(fn `FactorySettings`
  (returns (ReturnValue :type "SaveGame Object Reference"))
  (bind _returnvalue (`GameplayStatics.CreateSaveGameObject` (`self.SettingsSaveGameClass`)))
  (return _returnvalue))

(fn `Find Level Helpers`
  (returns (ReturnValue :type "Array of Object Object Reference"))
  (bind _outactors (`GameplayStatics.GetAllActorsOfClass` "/Game/LelouFW/Blueprint/Actor/LevelHelper/LelouFW_BP_Actor_LevelHelper.LelouFW_BP_Actor_LevelHelper_C"))
  (return _outactors))

(fn `FindLevelHelperActorsInLevel`
  (returns (ReturnValue :type "Array of Object Object Reference"))
  (bind _returnvalue (`self.Find Level Helpers`))
  (return _returnvalue))

(fn `GetAchievement`
  (returns (ReturnValue :type "SaveGame Object Reference"))
  (return (`self.AchievementSaveGame`)))

(fn `GetGameplay`
  (returns (ReturnValue :type "SaveGame Object Reference"))
  (bind _gameplaysavegame (`self.GameplaySaveGame`))
  (`/Engine/EditorBlueprintResources/StandardMacros.IsValid` _gameplaysavegame
    (:`Is Valid`
      _)
    (:`Is Not Valid`
      (bind _returnvalue (`self.FactoryGameplay`))
      (`self.SetGameplaySaveGame` _returnvalue)))
  (return _gameplaysavegame))

(fn `GetGameplaySaveGame`
  (returns (ReturnValue :type "SaveGame Object Reference"))
  (bind _returnvalue (`self.GetGameplay`))
  (return _returnvalue))

(fn `GetSettings`
  (returns (ReturnValue :type "SaveGame Object Reference"))
  (return (`self.SettingsSaveGame`)))

(fn `GetSettingsSaveGame`
  (returns (ReturnValue :type "SaveGame Object Reference"))
  (bind _returnvalue (`self.GetSettings`))
  (return _returnvalue))

(fn `HasGameplayTagInAchievement`
  (params (GameplayTag :type "GameplayTag Structure"))
  (returns (ReturnValue :type Boolean))
  (bind _returnvalue (`self.GetAchievement`))
  (bind _returnvalue_2 (message `/Game/LelouFW/Blueprint/SaveGame/Achievement/LelouFW_BPI_SaveGame_Achievement_Interface.HasAchievementGameplayTag` _returnvalue GameplayTag))
  (return _returnvalue_2))