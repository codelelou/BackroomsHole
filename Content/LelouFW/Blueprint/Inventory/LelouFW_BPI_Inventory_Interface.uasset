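; Blueprint interface for the LelouFW inventory system, declaring the calls used to drive an actor-based inventory.
; It covers showing, hiding and toggling the inventory and querying whether it is visible.
; Other functions add actors or actor classes, check membership with an index, list contents, cycle next or previous items and get or check the current one.
; All functions are empty declarations, leaving behavior to implementers.
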(fn `AddActorAtInventory`
  (params (Actor :type "Actor Object Reference"))
  (returns (Success :type Boolean) (Index :type Integer))
  (return false 0))

(fn `AddActorClassAtInventory`
  (params (ActorClass :type "Actor Class Reference")))

(fn `CheckCurrentInventoryActor`
  (params (Actor :type "Actor Object Reference"))
  (returns (ReturnValue :type Boolean))
  (return false))

(fn `GetCurrentInventoryActor`
  (returns (ReturnValue :type "Actor Object Reference"))
  (return null))

(fn `GetInventoryActors`
  (returns (ReturnValue :type "Array of Actor Object Reference"))
  (return))

(fn `HasActorAtInventory`
  (params (Actor :type "Actor Object Reference"))
  (returns (ReturnValue :type Boolean) (Index :type Integer))
  (return false 0))

(fn `HideInventory`)

(fn `InInventory`
  (params (Actor :type "Actor Object Reference"))
  (returns (ReturnValue :type Boolean))
  (return false))

(fn `IsShowInventory`
  (returns (ReturnValue :type Boolean))
  (return false))

(fn `NextInventoryItem`)

(fn `PrevInventoryItem`)

(fn `ShowInventory`)

(fn `ToggleInventory`)