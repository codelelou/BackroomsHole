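; Actor component that records an input mode as Game and UI values plus a widget to focus, without applying it to a player controller itself.
; SetInputMode captures the current state through GetInputMode before overwriting it, unless called as an undo, giving one level of history.
; Undo restores the captured Game and UI values but not the focus widget, guarded by an IsUndo flag that is never cleared.
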(event `SetInputMode`
  (params (Game :type Boolean) (UI :type Boolean) (InWidgetToFocus :type "Widget Object Reference") (Undo :type Boolean))
  (`|ExecutionSequence`
    (:`then_0`
      (if (not Undo)
        (`|ExecutionSequence`
          (:`then_0`
            (set `self.IsUndo` true))
          (:`then_1`
            (bind (_game _ui) (`self.GetInputMode`))))))
    (:`then_1`
      (`|ExecutionSequence`
        (:`then_0`
          (set `self.Game` Game))
        (:`then_1`
          (set `self.UI` UI))
        (:`then_2`
          (set `self.WidgetToFocus` InWidgetToFocus))))))

(event `Undo`
  (if (`self.ValidUndo`)
    (`self.SetInputMode` (stale `SetInputMode` _game) (stale `SetInputMode` _ui) null true)))

(fn `GetInputMode`
  (returns (Game :type Boolean) (UI :type Boolean) (WidgetToFocus :type "Widget Object Reference"))
  (return (`self.Game`) (`self.UI`) (`self.WidgetToFocus`)))

(fn `ValidUndo`
  (returns (ReturnValue :type Boolean))
  (return (`self.IsUndo`)))