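; Actor component that tracks character zoom and signals when a zoom-in reaches near maximum, likely for zoom-triggered events.
; On setup it binds to the zoom-changed event and uses direction and an FOV threshold to derive start, full-zoom and end phases.
; Chained DoOnce gates fire each phase once per zoom cycle.
; Full zoom sets a Finished flag and calls OnZoomFinished; start and end clear the flag, exposed through two getters.
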(event `self.ReceiveBeginPlay`
  (`self.Setup`))

(event `Setup`
  (`/Engine/EditorBlueprintResources/StandardMacros.DoOnce` false
    (:`Completed`
      (add `self.OnZoomChanged` (delegate `BindCharacterZoomingChanged`)))))

(event `BindCharacterZoomingChanged` :!signature `self.OnZoomChanged`
  (params (Zooming :type Boolean) (FOV :type "Float (double-precision)") (Direction :type "ETimelineDirection Enum" :default "Forward"))
  (switch `ETimelineDirection` Direction
    (:`Forward`
      (if Zooming
        (`|ExecutionSequence`
          (:`then_0`
            (`/Engine/EditorBlueprintResources/StandardMacros.DoOnce` false :!label _label ; Zoom開始時
              (:`Completed`
                (`|ExecutionSequence`
                  (:`then_0`
                    (`self.BindZoomStart`))
                  (:`then_1`
                    (goto _label_2 :!via `Reset`))
                  (:`then_2`
                    (goto _label_3 :!via `Reset`))))))
          (:`then_1`
            (if (< 0.9 FOV)
              (`/Engine/EditorBlueprintResources/StandardMacros.DoOnce` true :!label _label_2
                (:`Completed`
                  (`self.BindZoomFinished`))))))))
    (:`Backward`
      (`|ExecutionSequence`
        (:`then_0`
          (`/Engine/EditorBlueprintResources/StandardMacros.DoOnce` true :!label _label_3
            (:`Completed`
              (`self.BindZoomEnd`))))
        (:`then_1`
          (goto _label :!via `Reset`))))))

(event `SetFinished`
  (params (Finishing :type Boolean))
  (bind _output_get (set `self.Finished` Finishing))
  (if _output_get
    (`self.OnZoomFinished`)))

(event `BindZoomStart`
  (`self.SetFinished` false :!label _label_4))

(event `BindZoomEnd`
  (goto _label_4))

(event `BindZoomFinished`
  (`self.SetFinished` true))

(fn `Finishing`
  (returns (ReturnValue :type Boolean))
  (return (`self.Finished`)))

(fn `FinishingAtZoomEvent`
  (returns (ReturnValue :type Boolean))
  (return (`self.Finished`)))