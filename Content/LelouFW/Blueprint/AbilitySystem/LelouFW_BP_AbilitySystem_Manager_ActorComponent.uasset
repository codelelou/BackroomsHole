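; Actor component that manages a gameplay tag list for the ability system and restores abilities from save data.
; Send adds and removes tags, using a resettable DoOnce to raise one change event with a Save flag per change.
; TryActivateAbilityBySaveGame calls the empty LoadGameplayTags hook, then applies loaded tags as loose tags and grants and activates the supplied abilities, guarded by a DoOnce.
; SetLoadedGameplayTags stores loaded tags and appends them to the current list.
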(event `self.SendGameplayTags`
  (params (AddGameplayTag :type "GameplayTag Structure") (RemoveGameplayTag :type "GameplayTag Structure") (Save :type Boolean))
  (`self.Send` AddGameplayTag RemoveGameplayTag Save))

(event `TryActivateAbilityBySaveGame`
  (params (Actor :type "Actor Object Reference") (AbilitySystem :type "AbilitySystemComponent Object Reference") (GameplayAbilityClasses :type "Array of GameplayAbility Class Reference (by ref)"))
  ;[1 1 1] SaveGame (Load)
  (`/Engine/EditorBlueprintResources/StandardMacros.DoOnce` false :!label _label
    (:`Completed`
      (if (and (`KismetSystemLibrary.IsValid` AbilitySystem) (`KismetArrayLibrary.Array_IsNotEmpty` GameplayAbilityClasses))
        (`|ExecutionSequence`
          (:`then_0`
            (bind _returnvalue (`self.GetLoadedGameplayTags`)))
          (:`then_1`
            (if (`KismetArrayLibrary.Array_IsNotEmpty` _returnvalue)
              (for _array_element _returnvalue
                (`AbilitySystemBlueprintLibrary.AddLooseGameplayTags` Actor (`BlueprintGameplayTagLibrary.MakeGameplayTagContainerFromTag` _array_element)))
              (for _array_element_2 GameplayAbilityClasses
                (bind _returnvalue_2 (`AbilitySystemComponent.K2_GiveAbilityAndActivateOnce` AbilitySystem _array_element_2 0 -1))
                (`AbilitySystemComponent.TryActivateAbility` AbilitySystem _returnvalue_2 true)))))
        (else
          (goto _label :!via `Reset`))))))

(event `LoadGameplayTags`
  ;[1 1 1] SaveGame (Load)
)

(event `Send`
  (params (AddGameplayTag :type "GameplayTag Structure") (RemoveGameplayTag :type "GameplayTag Structure") (Save :type Boolean))
  (bind _currentgameplaytags (`self.CurrentGameplayTags`))
  (`|ExecutionSequence`
    (:`then_0`
      (if (`self.NotEmptyGameplayTag` AddGameplayTag)
        (bind _returnvalue (`KismetArrayLibrary.Array_Add` _currentgameplaytags AddGameplayTag))
        (if (<= 0 _returnvalue)
          (goto _label_2 :!via `Reset`))))
    (:`then_1`
      (if (`self.NotEmptyGameplayTag` RemoveGameplayTag)
        (bind _returnvalue_2 (`KismetArrayLibrary.Array_RemoveItem` _currentgameplaytags RemoveGameplayTag))
        (if _returnvalue_2
          (goto _label_2 :!via `Reset`))))
    (:`then_2`
      (`/Engine/EditorBlueprintResources/StandardMacros.DoOnce` true :!label _label_2
        (:`Completed`
          (`self.CallGameplayTagsChangedEventDispatcher` AddGameplayTag RemoveGameplayTag _currentgameplaytags Save))))))

(event `SetLoadedGameplayTags`
  (params (GameplayTags :type "Array of GameplayTag Structure"))
  (bind _output_get (set `self.LoadedGameplayTags` GameplayTags))
  (`KismetArrayLibrary.Array_Append` (`self.CurrentGameplayTags`) _output_get))

(event `CallGameplayTagsChangedEventDispatcher`
  (params (AddedGameplayTag :type "GameplayTag Structure") (RemovedGameplayTag :type "GameplayTag Structure") (CurrentGameplayTags :type "Array of GameplayTag Structure (by ref)") (Save :type Boolean))
  (`self.OnGameplayTagsChanged` AddedGameplayTag RemovedGameplayTag CurrentGameplayTags Save))

(fn `GetCurrentGameplayTags`
  (returns (ReturnValue :type "Array of GameplayTag Structure"))
  (return (`self.CurrentGameplayTags`)))

(fn `GetLoadedGameplayTags`
  (returns (ReturnValue :type "Array of GameplayTag Structure"))
  (`self.LoadGameplayTags`)
  (return (`self.LoadedGameplayTags`)))

(fn `Not Empty Gameplay Tag Container`
  (params (Value :type "GameplayTagContainer Structure (by ref)"))
  (returns (ReturnValue :type Boolean))
  (return (!= (`BlueprintGameplayTagLibrary.MakeLiteralGameplayTagContainer` (struct)) Value)))

(fn `NotEmptyGameplayTag`
  (params (Value :type "GameplayTag Structure (by ref)"))
  (returns (ReturnValue :type Boolean))
  (return (!= (struct) Value)))