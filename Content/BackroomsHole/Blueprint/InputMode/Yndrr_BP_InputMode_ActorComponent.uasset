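; Actor component Blueprint that switches the first player controller's input mode between game, UI, or both.
; Its SetInputMode event calls the parent, then picks Game and UI, Game Only, or UI Only from two flags, flushing input and passing the widget to focus.
; It shows the mouse cursor while UI is on and sends the controller a message that enables character control only when UI is off.
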(event `self.SetInputMode`
  (params (Game :type Boolean) (UI :type Boolean) (InWidgetToFocus :type "Widget Object Reference") (Undo :type Boolean))
  (bind _returnvalue (`GameplayStatics.GetPlayerController` 0))
  (`parent.SetInputMode` Game UI InWidgetToFocus false)
  (`|ExecutionSequence`
    (:`then_0`
      (if (and Game UI)
        (`WidgetBlueprintLibrary.SetInputMode_GameAndUIEx` _returnvalue InWidgetToFocus "DoNotLock" true true)
        (elif Game
          (`WidgetBlueprintLibrary.SetInputMode_GameOnly` _returnvalue true)
          (elif UI
            (`WidgetBlueprintLibrary.SetInputMode_UIOnlyEx` _returnvalue InWidgetToFocus "DoNotLock" true)))))
    (:`then_1`
      (set `PlayerController.bShowMouseCursor` UI _returnvalue))
    (:`then_2`
      (message `/Game/LelouFW/Blueprint/Controller/LelouFW_BPI_PlayerController_Interface.SetActiveCharacterControl` _returnvalue (not UI)))))