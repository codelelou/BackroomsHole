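; Animation model for closings such as hinged doors, sliding doors and drawers, covering open, close and locked motions.
; Door, Sliding and Locked timelines play at 1/Second rate, with closing played in reverse.
; Each update is broadcast through an event dispatcher with curve alphas and direction, leaving the actual movement to listeners.
; DoN and DoOnce counters double as state to derive the start, finished, reversing and locked-event flags sent along.
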(event `/Game/LelouFW/Blueprint/Closing/LelouFW_BPI_Closing_Model_Interface.OpenClosing`
  (params (Second :type "Float (double-precision)"))
  (`self.Open` Second))

(event `SlidingOpen`
  (params (Second :type "Float (double-precision)" :default 1.0))
  (bind _slidingtl (`self.SlidingTL`))
  ;[1 1 1] Slidng (引き戸・引出し向け)
  (`|ExecutionSequence`
    (:`then_0`
      (bind _counter (`/Engine/EditorBlueprintResources/StandardMacros.Do N` 1 :!label _label)) ; 0 = Close(Reverse) / 1 = Open
    )
    (:`then_1`
      (`TimelineComponent.SetPlayRate` _slidingtl (`self.GetPlayRateBySecond` Second _slidingtl)))
    (:`then_2`
      (bind (_direction _distance _angle) (`Timeline|SlidingTL` :!via `PlayFromStart` :!label _label_2)
        (:`Update`
          (`|ExecutionSequence`
            (:`then_0`
              (`self.CallSlidingTimelineEventDispatcher` (== 0 (stale _counter_2)) (== 2 (stale _counter_2)) (== 0 _counter) _direction _distance _angle :!label _label_3))
            (:`then_1`
              (`/Engine/EditorBlueprintResources/StandardMacros.DoOnce` false :!label _label_4
                (:`Completed`
                  (bind _counter_2 (`/Engine/EditorBlueprintResources/StandardMacros.Do N` 2 :!label _label_5)))))))
        (:`Finished`
          (`|ExecutionSequence`
            (:`then_0`
              (goto _label_5))
            (:`then_1`
              (goto _label_3))
            (:`then_2`
              (goto _label_5 :!via `Reset`))
            (:`then_3`
              (goto _label_4 :!via `Reset`))))))))

(event `/Game/LelouFW/Blueprint/Closing/LelouFW_BPI_Closing_Model_Interface.CloseClosing`
  (params (Second :type "Float (double-precision)"))
  (`self.Close` Second))

(event `SlidingClose`
  (params (Second :type "Float (double-precision)" :default 1.0))
  (bind _slidingtl (`self.SlidingTL`))
  ;[1 1 1] Slidng (引き戸・引出し向け)
  (`|ExecutionSequence`
    (:`then_0`
      (goto _label))
    (:`then_1`
      (`TimelineComponent.SetPlayRate` _slidingtl (`self.GetPlayRateBySecond` Second _slidingtl)))
    (:`then_2`
      (goto _label_2 :!via `ReverseFromEnd`))))

(event `/Game/LelouFW/Blueprint/Closing/LelouFW_BPI_Closing_Model_Interface.LockedClosing`
  (`self.Locked` 1.0))

(event `/Game/LelouFW/Blueprint/Closing/LelouFW_BPI_Closing_Model_Interface.SlidingClosing`
  (params (Reverse :type Boolean) (Second :type "Float (double-precision)"))
  (`self.Sliding` Reverse Second))

(event `Open`
  (params (Second :type "Float (double-precision)" :default 0.5))
  (bind _doortl (`self.DoorTL`))
  ;[1 1 1] Hinge (引き戸・引出しなどは「Sliding」を使用）
  (`|ExecutionSequence`
    (:`then_0`
      (bind _counter (`/Engine/EditorBlueprintResources/StandardMacros.Do N` 1 :!label _label_6)) ; 0 = Close(Reverse) / 1 = Open
    )
    (:`then_1`
      (`TimelineComponent.SetPlayRate` _doortl (`self.GetPlayRateBySecond` Second _doortl)))
    (:`then_2`
      (bind (_direction _panelangle _knobangle) (`Timeline|DoorTL` :!via `PlayFromStart` :!label _label_7)
        (:`Update`
          (`|ExecutionSequence`
            (:`then_0`
              (`self.CallDoorTimelineEventDispatcher` (== 0 (stale _counter_2)) (== 2 (stale _counter_2)) (== _counter 0) _direction _panelangle _knobangle :!label _label_8))
            (:`then_1`
              (`/Engine/EditorBlueprintResources/StandardMacros.DoOnce` false :!label _label_9
                (:`Completed`
                  (bind _counter_2 (`/Engine/EditorBlueprintResources/StandardMacros.Do N` 2 :!label _label_10)))))))
        (:`Finished`
          (`|ExecutionSequence`
            (:`then_0`
              (goto _label_10))
            (:`then_1`
              (goto _label_8))
            (:`then_2`
              (goto _label_10 :!via `Reset`))
            (:`then_3`
              (goto _label_9 :!via `Reset`))))))))

(event `Sliding`
  (params (Reverse :type Boolean) (Second :type "Float (double-precision)"))
  ;[1 1 1] Slidng (引き戸・引出し向け)
  (if Reverse
    (`self.SlidingClose` Second)
    (else
      (`self.SlidingOpen` Second))))

(event `CallSlidingTimelineEventDispatcher`
  (params (Start :type Boolean) (Finished :type Boolean) (IsReversing :type Boolean) (Direction :type "ETimelineDirection Enum" :default "Forward") (DistanceAlpha :type "Float (double-precision)") (AngleAlpha :type "Float (double-precision)"))
  ;[1 1 1] Slidng (引き戸・引出し向け)
  (`self.OnSlidingTimeline` Start Finished IsReversing Direction DistanceAlpha AngleAlpha))

(event `Close`
  (params (Scond :type "Float (double-precision)" :default 0.5))
  (bind _doortl (`self.DoorTL`))
  ;[1 1 1] Hinge (引き戸・引出しなどは「Sliding」を使用）
  (`|ExecutionSequence`
    (:`then_0`
      (goto _label_6 :!via `Reset`))
    (:`then_1`
      (`TimelineComponent.SetPlayRate` _doortl (`self.GetPlayRateBySecond` Scond _doortl)))
    (:`then_2`
      (goto _label_7 :!via `ReverseFromEnd`))))

(event `CallDoorTimelineEventDispatcher`
  (params (Start :type Boolean) (Finished :type Boolean) (IsReversing :type Boolean) (Direction :type "ETimelineDirection Enum" :default "Forward") (PanelAngle :type "Float (double-precision)") (KnobAngle :type "Float (double-precision)"))
  ;[1 1 1] Hinge (引き戸・引出しなどは「Sliding」を使用）
  (`self.OnDoorTimeline` Start Finished IsReversing Direction PanelAngle KnobAngle))

(event `Locked`
  (params (Second :type "Float (double-precision)" :default 1.0))
  (bind _lockedtl (`self.LockedTL`))
  ;[1 1 1] Locked
  (`TimelineComponent.SetPlayRate` _lockedtl (`self.GetPlayRateBySecond` Second _lockedtl))
  (bind (_direction _hingeangle _knobangle) (`Timeline|LockedTL` :!via `PlayFromStart`)
    (:`Update`
      (`|ExecutionSequence`
        (:`then_0`
          (`self.CallLockedTimelineEventDispatcher` (== 0 (stale _counter)) (== 2 (stale _counter)) _direction (< 0 (stale _counter_2)) _hingeangle _knobangle :!label _label_11))
        (:`then_1`
          (`/Engine/EditorBlueprintResources/StandardMacros.DoOnce` false :!label _label_12
            (:`Completed`
              (bind _counter (`/Engine/EditorBlueprintResources/StandardMacros.Do N` 2 :!label _label_13)))))
        (:`then_2`
          (goto _label_14 :!via `Reset`))))
    (:`Finished`
      (`|ExecutionSequence`
        (:`then_0`
          (goto _label_13))
        (:`then_1`
          (goto _label_11))
        (:`then_2`
          (goto _label_13 :!via `Reset`))
        (:`then_3`
          (goto _label_12 :!via `Reset`))))
    (:`LockedEvent`
      (bind _counter_2 (`/Engine/EditorBlueprintResources/StandardMacros.Do N` 1 :!label _label_14)))))

(event `CallLockedTimelineEventDispatcher`
  (params (Start :type Boolean) (Finished :type Boolean) (Direction :type "ETimelineDirection Enum" :default "Forward") (Event :type Boolean) (HingeAngleAlpha :type "Float (double-precision)") (KnobAngleAlpha :type "Float (double-precision)"))
  ;[1 1 1] Locked
  (`self.OnLockedTimeline` Start Finished Direction Event HingeAngleAlpha KnobAngleAlpha))

(fn `GetPlayRateBySecond`
  (params (Second :type "Float (double-precision)" :default 1.0) (Timeline :type "TimelineComponent Object Reference"))
  (returns (ReturnValue :type "Float (double-precision)"))
  (return (/ 1.0 Second)))

(fn `UserConstructionScript`)