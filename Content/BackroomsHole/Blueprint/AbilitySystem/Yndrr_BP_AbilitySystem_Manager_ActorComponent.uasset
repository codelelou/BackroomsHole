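; Ability system manager component that adds save-game persistence for gameplay tags to its parent class.
; On tag changes, it writes added and removed tags to the GameInstance's gameplay save, saves through player 0's PlayerState save component when flagged, then calls the parent.
; On load, it runs the parent logic, then applies the saved tags once through a DoOnce.
; Save access goes through message calls.
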(event `self.CallGameplayTagsChangedEventDispatcher`
  (params (AddedGameplayTag :type "GameplayTag Structure") (RemovedGameplayTag :type "GameplayTag Structure") (CurrentGameplayTags :type "Array of GameplayTag Structure (by ref)") (Save :type Boolean))
  (`|ExecutionSequence`
    (:`then_0`
      (bind _returnvalue (message `/Game/LelouFW/Blueprint/GameInstance/LelouFW_BPI_GameInstance_Gameplay_Interface.GetGameplaySaveGame` (`GameplayStatics.GetGameInstance`)))
      (`|ExecutionSequence`
        (:`then_0`
          (message `/Game/LelouFW/Blueprint/SaveGame/Gameplay/LelouFW_BPI_SaveGame_Gameplay_Interface.UpdateGameplayTagsInSaveGame` _returnvalue AddedGameplayTag RemovedGameplayTag))
        (:`then_1`
          (if Save
            (bind _returnvalue_2 (message `/Game/LelouFW/Blueprint/PlayerState/LelouFW_BPI_PlayerState_Interface.GetSaveGameComponent` (`GameplayStatics.GetPlayerState` 0)))
            (message `/Game/LelouFW/Blueprint/SaveGame/LelouFW_BPI_SaveGame_ActorComponent_Interface.SaveGameplaySaveGame` _returnvalue_2 _returnvalue "" 0)))))
    (:`then_1`
      (`parent.CallGameplayTagsChangedEventDispatcher` AddedGameplayTag RemovedGameplayTag CurrentGameplayTags Save))))

(event `self.LoadGameplayTags`
  (`parent.LoadGameplayTags`)
  (`/Engine/EditorBlueprintResources/StandardMacros.DoOnce` false
    (:`Completed`
      (bind _returnvalue (message `/Game/LelouFW/Blueprint/GameInstance/LelouFW_BPI_GameInstance_Gameplay_Interface.GetGameplaySaveGame` (`GameplayStatics.GetGameInstance`)))
      (bind _returnvalue_2 (message `/Game/LelouFW/Blueprint/SaveGame/Gameplay/LelouFW_BPI_SaveGame_Gameplay_Interface.GetGameplayTagsInSaveGame` _returnvalue))
      (`self.SetLoadedGameplayTags` _returnvalue_2))))