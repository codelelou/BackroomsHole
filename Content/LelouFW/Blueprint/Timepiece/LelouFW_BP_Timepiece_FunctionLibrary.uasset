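; Blueprint function library for timepieces that converts a Timespan into analog clock hand angles and formatted display text.
; Hour, minute and second helpers map time into a given angle range, with a 12-hour dial and reversed mapping for negative spans, and GetAngleForAnalogClock returns all three.
; Second angles include milliseconds for smooth motion, while minute angles step in whole minutes.
; FormatTimespanText fills a format pattern with zero-padded time fields.
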(fn `FormatTimespanText`
  (params (Timespan :type "Timespan Structure") (Format :type Text :default "NSLOCTEXT(\"[A8B4CFD14ABE7A8A2FF405959C4099BE]\", \"5094DECC4B674AC717826D9504B61462\", \"{Hours}:{Minutes}.{Seconds}\")"))
  (returns (ReturnValue :type Text))
  (bind (_days _hours _minutes _seconds _milliseconds) (`KismetMathLibrary.BreakTimespan` Timespan))
  (return (`|FormatText` Format (`KismetTextLibrary.Conv_IntToText` _days false false 2) (`KismetTextLibrary.Conv_IntToText` _hours false false 2) (`KismetTextLibrary.Conv_IntToText` _minutes false false 2) (`KismetTextLibrary.Conv_IntToText` _seconds false false 2) (`KismetTextLibrary.Conv_IntToText` _milliseconds false false 3))))

(fn `GetAngleForAnalogClock`
  (params (Time :type "Timespan Structure") (MinAngle :type "Float (double-precision)") (MaxAngle :type "Float (double-precision)" :default 360.0))
  (returns (HourAngle :type "Float (double-precision)") (MinuteAngle :type "Float (double-precision)") (SecondAngle :type "Float (double-precision)"))
  (return (`self.GetHourAngle` Time MinAngle MaxAngle) (`self.GetMinuteAngle` Time MinAngle MaxAngle) (`self.GetSecondAngle` Time MinAngle MaxAngle)))

(fn `GetHourAngle`
  (params (Time :type "Timespan Structure") (MinAngle :type "Float (double-precision)") (MaxAngle :type "Float (double-precision)" :default 360.0))
  (returns (ReturnValue :type "Float (double-precision)"))
  (bind (_days _hours _minutes _seconds _milliseconds) (`KismetMathLibrary.BreakTimespan` Time))
  (bind _returnvalue (* 43200.0 2.0))
  (bind _returnvalue_2 (`KismetMathLibrary.GetTotalSeconds` (`KismetMathLibrary.MakeTimespan` 0 _hours _minutes _seconds _milliseconds)))
  (bind _returnvalue_3 (`KismetMathLibrary.Abs` _returnvalue_2))
  (if (<= (`KismetMathLibrary.MakeTimespan` 0) Time)
    (if (<= 12 _hours)
      (return (`KismetMathLibrary.MapRangeClamped` _returnvalue_2 43200.0 _returnvalue MinAngle MaxAngle))
      (else
        (return (`KismetMathLibrary.MapRangeClamped` _returnvalue_2 0.0 43200.0 MinAngle MaxAngle))))
    (elif (< -12 _hours)
      (return (`KismetMathLibrary.MapRangeClamped` _returnvalue_3 43200.0 0.0 MinAngle MaxAngle))
      (else
        (return (`KismetMathLibrary.MapRangeClamped` _returnvalue_3 _returnvalue 43200.0 MinAngle MaxAngle))))))

(fn `GetMinuteAngle`
  (params (Time :type "Timespan Structure") (MinAngle :type "Float (double-precision)") (MaxAngle :type "Float (double-precision)" :default 360.0))
  (returns (ReturnValue :type "Float (double-precision)"))
  (bind (_days _hours _minutes) (`KismetMathLibrary.BreakTimespan` Time))
  (bind _returnvalue (`KismetMathLibrary.Conv_IntToDouble` _minutes))
  (if (<= 0 _minutes)
    (return (`KismetMathLibrary.MapRangeClamped` _returnvalue 0.0 60.0 MinAngle MaxAngle))
    (else
      (return (`KismetMathLibrary.MapRangeClamped` (`KismetMathLibrary.Abs` _returnvalue) 60.0 0.0 MinAngle MaxAngle)))))

(fn `GetSecondAngle`
  (params (Time :type "Timespan Structure") (MinAngle :type "Float (double-precision)") (MaxAngle :type "Float (double-precision)" :default 360.0))
  (returns (ReturnValue :type "Float (double-precision)"))
  (bind (_days _hours _minutes _seconds _milliseconds) (`KismetMathLibrary.BreakTimespan` Time))
  (bind _returnvalue (+ _seconds (/ (`KismetMathLibrary.Conv_IntToDouble` _milliseconds) 1000.0)))
  (if (<= 0 _seconds)
    (return (`KismetMathLibrary.MapRangeClamped` _returnvalue 0.0 60.0 MinAngle MaxAngle))
    (else
      (return (`KismetMathLibrary.MapRangeClamped` (`KismetMathLibrary.Abs` _returnvalue) 60.0 0.0 MinAngle MaxAngle)))))