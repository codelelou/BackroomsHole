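; Blueprint Interface for the HUD in BackroomsHole, declaring getters for the game's individual HUD elements.
; The functions cover dialogue, notice, action, pause, actor viewer, inventory, zoomed event, reticle, zooming text and save menu.
; It holds only empty declarations, leaving the lookup logic to whichever class implements it.
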(fn `GetActionInHUD`
  (returns (ReturnValue :type "UserWidget Object Reference"))
  (return null))

(fn `GetActorViewerInHUD`
  (returns (ReturnValue :type "UserWidget Object Reference"))
  (return null))

(fn `GetDialogueInHUD`
  (returns (ReturnValue :type "UserWidget Object Reference"))
  (return null))

(fn `GetInventoryInHUD`
  (returns (ReturnValue :type "UserWidget Object Reference"))
  (return null))

(fn `GetNoticeInHUD`
  (returns (ReturnValue :type "UserWidget Object Reference"))
  (return null))

(fn `GetPauseInHUD`
  (returns (ReturnValue :type "UserWidget Object Reference"))
  (return null))

(fn `GetReticleInHUD`
  (returns (ReturnValue :type "UserWidget Object Reference"))
  (return null))

(fn `GetSaveMenuInHUD`
  (returns (ReturnValue :type "UserWidget Object Reference"))
  (return null))

(fn `GetZoomedEventInHUD`
  (returns (ReturnValue :type "UserWidget Object Reference"))
  (return null))

(fn `GetZoomingTextInHUD`
  (returns (ReturnValue :type "UserWidget Object Reference"))
  (return null))