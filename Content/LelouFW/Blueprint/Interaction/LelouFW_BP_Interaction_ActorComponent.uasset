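; Interaction actor component that detects which registered areas the player pawn is inside and which interaction targets the camera faces.
; Begin and end overlaps on the registered overlap areas update the current list, start or pause a looping 30 Hz timer, and fire a dispatcher.
; Each timer tick filters orientation areas by pawn distance and camera look angle, using a Gate and count comparison to broadcast interactable-area changes.
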(event `/Game/LelouFW/Blueprint/Interaction/LelouFW_BPI_Interaction_ActorComponent_Interface.AddInteractionOverlapArea`
  (params (Area :type "PrimitiveComponent Object Reference"))
  (`self.AddOverlapArea` Area))

(event `AddOrientationAreas`
  (params (OrientationAreas :type "Array of SceneComponent Object Reference (by ref)"))
  ;[1 1 1] Orientation
  (`KismetArrayLibrary.Array_Append` (`self.OrientationAreas`) OrientationAreas))

(event `self.ReceiveTick`
  (params (DeltaSeconds :type "Float (single-precision)")))

(event `/Game/LelouFW/Blueprint/Interaction/LelouFW_BPI_Interaction_ActorComponent_Interface.AddInteractionOverlapAreas`
  (params (Areas :type "Array of PrimitiveComponent Object Reference (by ref)"))
  (`self.AddOverlapAreas` Areas))

(event `AddOrientationArea`
  (params (OrientationArea :type "SceneComponent Object Reference (by ref)"))
  ;[1 1 1] Orientation
  (`KismetArrayLibrary.Array_AddUnique` (`self.OrientationAreas`) OrientationArea))

(event `/Game/LelouFW/Blueprint/Interaction/LelouFW_BPI_Interaction_ActorComponent_Interface.AddInteractionOrientationArea`
  (params (Area :type "SceneComponent Object Reference"))
  (`self.AddOrientationArea` Area))

(event `SetOrientationDistance`
  (params (Value :type "Float (double-precision)"))
  (set `self.OrientationDistance` Value))

(event `Start`
  ;[1 1 1] Orientation
  (if (`self.IsOverlapping`)
    (`|ExecutionSequence`
      (:`then_0`
        (`/Engine/EditorBlueprintResources/StandardMacros.DoOnce` false :!label _label
          (:`Completed`
            (bind _returnvalue (`KismetSystemLibrary.K2_SetTimerDelegate` (delegate `Watch`) (/ 1.0 30.0) true)))))
      (:`then_1`
        (if (`KismetSystemLibrary.K2_IsTimerPausedHandle` _returnvalue)
          (`KismetSystemLibrary.K2_UnPauseTimerHandle` _returnvalue))))
    (else
      (`self.Pause`))))

(event `/Game/LelouFW/Blueprint/Interaction/LelouFW_BPI_Interaction_ActorComponent_Interface.AddInteractionOrientationAreas`
  (params (Areas :type "Array of SceneComponent Object Reference (by ref)"))
  (`self.AddOrientationAreas` Areas))

(event `SetOrientationRange`
  (params (Value :type "Float (double-precision)"))
  (set `self.OrientationRange` Value))

(event `Stop`
  ;[1 1 1] Orientation
  (`KismetSystemLibrary.K2_ClearAndInvalidateTimerHandle` (stale `Start` _returnvalue))
  (goto _label :!via `Reset`))

(event `/Game/LelouFW/Blueprint/Interaction/LelouFW_BPI_Interaction_ActorComponent_Interface.CheckInteractionOverlapAreas`
  (`self.CheckOverlappedAreas`))

(event `AddOverlapArea`
  (params (OverlapArea :type "PrimitiveComponent Object Reference (by ref)"))
  ;[1 1 1] Overlap
  (bind _returnvalue (`KismetArrayLibrary.Array_AddUnique` (`self.OverlapAreas`) OverlapArea))
  (if (<= 0 _returnvalue)
    (`self.SetupOverlapArea` OverlapArea)))

(event `Pause`
  ;[1 1 1] Orientation
  (`self.ClearCurrentInteractAreas`)
  (`|ExecutionSequence`
    (:`then_0`
      (if (`KismetSystemLibrary.K2_IsTimerActiveHandle` (stale `Start` _returnvalue))
        (`KismetSystemLibrary.K2_PauseTimerHandle` (stale `Start` _returnvalue))))
    (:`then_1`
      (if (!= (`KismetArrayLibrary.Array_Length` (stale `CallChangedInteractAreasEventDispatcher` InteractAreas)) (`KismetArrayLibrary.Array_Length` (`self.CurrentInteractAreas`)))
        (`self.CallChangedInteractAreasEventDispatcher` (`|MakeArray`))))))

(event `AddOverlapAreas`
  (params (OverlapAreas :type "Array of PrimitiveComponent Object Reference (by ref)"))
  ;[1 1 1] Overlap
  (for _array_element OverlapAreas
    (`self.AddOverlapArea` _array_element)))

(event `CallChangedInteractAreasEventDispatcher`
  (params (InteractAreas :type "Array of SceneComponent Object Reference (by ref)"))
  ;[1 1 1] Orientation
  (`self.OnChangedInteractAreas` InteractAreas))

(event `CheckOverlappedAreas`
  ;[1 1 1] Overlap
  (bind _returnvalue (`self.GetInteracter`))
  (for _array_element (`self.OverlapAreas`)
    (if (`PrimitiveComponent.IsOverlappingActor` _array_element _returnvalue)
      (`self.AddCurrentOverlappedArea` _array_element))))

(event `Watch`
  (bind _currentinteractareas (`self.CurrentInteractAreas`))
  ;[1 1 1] Orientation
  (`|ExecutionSequence`
    (:`then_0`
      (`self.ClearCurrentInteractAreas`))
    (:`then_1`
      (goto _label_2 :!via `Close`))
    (:`then_2`
      (bind _returnvalue (`self.GetOrientationAreas`))
      (for _array_element _returnvalue
        (if (`self.CheckInteract` _array_element)
          (`|ExecutionSequence`
            (:`then_0`
              (`KismetArrayLibrary.Array_AddUnique` _currentinteractareas _array_element))
            (:`then_1`
              (if (not (`KismetArrayLibrary.Array_Contains` (stale `CallChangedInteractAreasEventDispatcher` InteractAreas) _array_element))
                (goto _label_2 :!via `Open`)))))))
    (:`then_3`
      (if (not (!= (`KismetArrayLibrary.Array_Length` (stale `CallChangedInteractAreasEventDispatcher` InteractAreas)) (`KismetArrayLibrary.Array_Length` _currentinteractareas)))
        (`/Engine/EditorBlueprintResources/StandardMacros.Gate` true :!label _label_2
          (:`Exit`
            _)))
      (`self.CallChangedInteractAreasEventDispatcher` _currentinteractareas))))

(event `SetupOverlapArea`
  (params (OverlapArea :type "PrimitiveComponent Object Reference (by ref)"))
  ;[1 1 1] Overlap
  (add `PrimitiveComponent.OnComponentBeginOverlap` OverlapArea (delegate `BindOverlapAreaBeginOverlap`))
  (add `PrimitiveComponent.OnComponentEndOverlap` OverlapArea (delegate `BindOverlapAreaEndOverlap`)))

(event `ClearCurrentInteractAreas`
  ;[1 1 1] Orientation
  (`KismetArrayLibrary.Array_Clear` (`self.CurrentInteractAreas`)))

(event `BindOverlapAreaBeginOverlap`
  (params (OverlappedComponent :type "PrimitiveComponent Object Reference") (OtherActor :type "Actor Object Reference") (OtherComp :type "PrimitiveComponent Object Reference") (OtherBodyIndex :type Integer) (bFromSweep :type Boolean) (SweepResult :type "HitResult Structure (by ref)"))
  ;[1 1 1] Overlap
  (if (`self.CheckOverlap` OtherActor)
    (`self.AddCurrentOverlappedArea` OverlappedComponent)))

(event `BindOverlapAreaEndOverlap`
  (params (OverlappedComponent :type "PrimitiveComponent Object Reference") (OtherActor :type "Actor Object Reference") (OtherComp :type "PrimitiveComponent Object Reference") (OtherBodyIndex :type Integer))
  ;[1 1 1] Overlap
  (if (`self.CheckOverlap` OtherActor)
    (bind _returnvalue (`KismetArrayLibrary.Array_RemoveItem` (`self.CurrentOverlappedAreas`) OverlappedComponent))
    (if _returnvalue
      (`|ExecutionSequence`
        (:`then_0`
          (`self.Pause`))
        (:`then_1`
          (`self.CallChangedOverlapedArea` null))))))

(event `AddCurrentOverlappedArea`
  (params (OverlappedArea :type "PrimitiveComponent Object Reference"))
  ;[1 1 1] Overlap
  (if (`self.ContainOverlapAreas` OverlappedArea)
    (bind _returnvalue (`KismetArrayLibrary.Array_AddUnique` (`self.CurrentOverlappedAreas`) OverlappedArea))
    (if (<= 0 _returnvalue)
      (`|ExecutionSequence`
        (:`then_0`
          (`self.Start`))
        (:`then_1`
          (`self.CallChangedOverlapedArea` OverlappedArea))))))

(event `CallChangedOverlapedArea`
  (params (NewArea :type "PrimitiveComponent Object Reference"))
  ;[1 1 1] Overlap
  (bind _returnvalue (`self.GetCurrentOverlappedAreas`))
  (`self.OnChangedOverlappedAreas` NewArea _returnvalue))

(fn `CheckInteract`
  (params (Target :type "SceneComponent Object Reference"))
  (returns (ReturnValue :type Boolean))
  (bind _returnvalue (`SceneComponent.K2_GetComponentLocation` Target))
  (bind (_startforward _startlocation) (`self.GetCameraInfo`))
  (bind _returnvalue_2 (`self.GetInteracter`))
  (if (`self.CheckOrientationDistance` (`Actor.K2_GetActorLocation` _returnvalue_2) _returnvalue (`self.OrientationDistance`))
    (return (`self.CheckOrientationAngle` _startforward _startlocation _returnvalue (`self.OrientationRange`)))
    (else
      (return false))))

(fn `CheckInteractionCurrentOrientation`
  (params (Targets :type "Array of SceneComponent Object Reference (by ref)"))
  (returns (ReturnValue :type Boolean))
  (for _array_element Targets
    (if (`KismetArrayLibrary.Array_Contains` (`self.CurrentInteractAreas`) _array_element)
      (`|ExecutionSequence`
        (:`then_0`
          (return true))
        (:`then_1`
          (break)))))
  (return false))

(fn `CheckOrientationAngle`
  (params (StartForward :type "Vector Structure") (StartLocation :type "Vector Structure (by ref)") (TargetLocation :type "Vector Structure (by ref)") (Range :type "Float (double-precision)" :default 10.0))
  (returns (ReturnValue :type Boolean))
  (return (< (`KismetMathLibrary.DegAcos` (`KismetMathLibrary.Dot_VectorVector` StartForward (`KismetMathLibrary.GetForwardVector` (`KismetMathLibrary.FindLookAtRotation` StartLocation TargetLocation)))) Range)))

(fn `CheckOrientationDistance`
  (params (Player :type "Vector Structure") (Target :type "Vector Structure") (Distance :type "Float (double-precision)" :default 200.0))
  (returns (ReturnValue :type Boolean))
  (return (< (`KismetMathLibrary.VSize` (- Player Target)) Distance)))

(fn `CheckOverlap`
  (params (OtherActor :type "Actor Object Reference"))
  (returns (ReturnValue :type Boolean))
  (bind _returnvalue (`self.GetInteracter`))
  (return (== _returnvalue OtherActor)))

(fn `ContainOverlapAreas`
  (params (Area :type "PrimitiveComponent Object Reference (by ref)"))
  (returns (ReturnValue :type Boolean))
  (return (`KismetArrayLibrary.Array_Contains` (`self.OverlapAreas`) Area)))

(fn `GetCameraInfo`
  (returns (StartForward :type "Vector Structure") (StartLocation :type "Vector Structure"))
  (bind _returnvalue (`GameplayStatics.GetPlayerCameraManager` 0))
  (return (`Actor.GetActorForwardVector` _returnvalue) (`PlayerCameraManager.GetCameraLocation` _returnvalue)))

(fn `GetCurrentOverlappedAreas`
  (returns (ReturnValue :type "Array of PrimitiveComponent Object Reference"))
  (return (`self.CurrentOverlappedAreas`)))

(fn `GetInteracter`
  (returns (ReturnValue :type "Actor Object Reference"))
  (return (`GameplayStatics.GetPlayerPawn` 0)))

(fn `GetInteractionCurrentOverlappedAreas`
  (returns (ReturnValue :type "Array of PrimitiveComponent Object Reference"))
  (bind _returnvalue (`self.GetCurrentOverlappedAreas`))
  (return _returnvalue))

(fn `GetInteractionOrientationAreas`
  (returns (ReturnValue :type "Array of SceneComponent Object Reference"))
  (bind _returnvalue (`self.GetOrientationAreas`))
  (return _returnvalue))

(fn `GetOrientationAreas`
  (returns (ReturnValue :type "Array of SceneComponent Object Reference"))
  (return (`self.OrientationAreas`)))

(fn `IsInteractingOfInteraction`
  (returns (ReturnValue :type Boolean))
  (return (`KismetArrayLibrary.Array_IsNotEmpty` (`self.CurrentInteractAreas`))))

(fn `IsOverlapping`
  (returns (ReturnValue :type Boolean))
  (bind _returnvalue (`self.GetCurrentOverlappedAreas`))
  (return (`KismetArrayLibrary.Array_IsNotEmpty` _returnvalue)))

(fn `IsOverlappingOfInteraction`
  (returns (ReturnValue :type Boolean))
  (return (`self.IsOverlapping`)))