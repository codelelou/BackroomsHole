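; HUD Blueprint that creates and serves the game's UI widgets, such as dialogue, inventory, pause, save menu, notices and reticle.
; FactoryUserWidget lazily creates one instance per class, caches it in the UserWidgets map and optionally adds it to viewport or player screen.
; Typed getters wrap the factory with each widget's placement, raising Z-order for notice, pause and save menu.
; ShowDialogue passes a DataTable to the dialogue widget with typewriter effect enabled.
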(event `self.ReceiveBeginPlay`)

(event `/Game/LelouFW/Blueprint/HUD/LelouFW_BPI_HUD_Dialogue_Interface.ShowDialogue`
  (params (DataTable :type "DataTable Object Reference") (Auto :type Boolean))
  (bind _returnvalue (`self.FactoryUserWidget` "/Game/BackroomsHole/Blueprint/Dialogue/Yndrr_WBP_Dialogue.Yndrr_WBP_Dialogue_C"))
  (message `/Game/LelouFW/Blueprint/Dialogue/LelouFW_BPI_Dialogue_Interface.ShowDialogue` _returnvalue DataTable Auto true))

(fn `FactoryUserWidget`
  (params (Class :type "UserWidget Class Reference") (AddToViewport :type Boolean) (AddToPlayerScreen :type Boolean) (ZOrder :type Integer))
  (returns (ReturnValue :type "UserWidget Object Reference"))
  (bind _userwidgets (`self.UserWidgets`))
  (bind (_value _returnvalue) (`BlueprintMapLibrary.Map_Find` _userwidgets Class))
  (if (`KismetSystemLibrary.IsValidClass` Class)
    (if _returnvalue
      (return _value)
      (else
        (bind _returnvalue_2 (`|CreateWidget` Class))
        (`|ExecutionSequence`
          (:`then_0`
            (`BlueprintMapLibrary.Map_Add` _userwidgets Class _returnvalue_2))
          (:`then_1`
            (if AddToViewport
              (`UserWidget.AddToViewport` _returnvalue_2 ZOrder)
              (elif AddToPlayerScreen
                (`UserWidget.AddToPlayerScreen` _returnvalue_2 ZOrder))))
          (:`then_2`
            (return _returnvalue_2)))))
    (else
      (return null))))

(fn `GetActionInHUD`
  (returns (ReturnValue :type "UserWidget Object Reference"))
  (bind _returnvalue (`self.FactoryUserWidget` "/Game/BackroomsHole/Blueprint/Action/Yndrr_WBP_Action.Yndrr_WBP_Action_C" false true))
  (return _returnvalue))

(fn `GetActorViewerInHUD`
  (returns (ReturnValue :type "UserWidget Object Reference"))
  (bind _returnvalue (`self.FactoryUserWidget` "/Game/BackroomsHole/Blueprint/ActorViewer/Yndrr_WBP_ActorViewer.Yndrr_WBP_ActorViewer_C" false true))
  (return _returnvalue))

(fn `GetDialogueInHUD`
  (returns (ReturnValue :type "UserWidget Object Reference"))
  (bind _returnvalue (`self.FactoryUserWidget` "/Game/BackroomsHole/Blueprint/Dialogue/Yndrr_WBP_Dialogue.Yndrr_WBP_Dialogue_C" false true))
  (return _returnvalue))

(fn `GetInventoryInHUD`
  (returns (ReturnValue :type "UserWidget Object Reference"))
  (bind _returnvalue (`self.FactoryUserWidget` "/Game/BackroomsHole/Blueprint/Inventory/Yndrr_WBP_Inventory.Yndrr_WBP_Inventory_C" false true))
  (return _returnvalue))

(fn `GetNoticeInHUD`
  (returns (ReturnValue :type "UserWidget Object Reference"))
  (bind _returnvalue (`self.FactoryUserWidget` "/Game/BackroomsHole/Blueprint/Notice/Yndrr_WBP_Notice.Yndrr_WBP_Notice_C" false true 900))
  (return _returnvalue))

(fn `GetPauseInHUD`
  (returns (ReturnValue :type "UserWidget Object Reference"))
  (bind _returnvalue (`self.FactoryUserWidget` "/Game/BackroomsHole/Blueprint/Widget/UserWidget/Pause/Yndrr_WBP_Pause.Yndrr_WBP_Pause_C" false true 1000))
  (return _returnvalue))

(fn `GetReticleInHUD`
  (returns (ReturnValue :type "UserWidget Object Reference"))
  (bind _returnvalue (`self.FactoryUserWidget` "/Game/BackroomsHole/Blueprint/Widget/UserWidget/Reticle/Yndrr_WBP_Reticle.Yndrr_WBP_Reticle_C" false true))
  (return _returnvalue))

(fn `GetSaveMenuInHUD`
  (returns (ReturnValue :type "UserWidget Object Reference"))
  (bind _returnvalue (`self.FactoryUserWidget` "/Game/BackroomsHole/Blueprint/Widget/UserWidget/GameplaySaveGame/Yndrr_WBP_GameplaySaveGame_Save.Yndrr_WBP_GameplaySaveGame_Save_C" true false 1200))
  (return _returnvalue))

(fn `GetZoomedEventInHUD`
  (returns (ReturnValue :type "UserWidget Object Reference"))
  (bind _returnvalue (`self.FactoryUserWidget` "/Game/BackroomsHole/Blueprint/ZoomEvent/Yndrr_UW_ZoomEvent.Yndrr_UW_ZoomEvent_C" false true))
  (return _returnvalue))

(fn `GetZoomingTextInHUD`
  (returns (ReturnValue :type "UserWidget Object Reference"))
  (bind _returnvalue (`self.FactoryUserWidget` "/Game/BackroomsHole/Blueprint/ZoomingText/Yndrr_UW_ZoomingText.Yndrr_UW_ZoomingText_C" true))
  (return _returnvalue))

(fn `UserConstructionScript`)