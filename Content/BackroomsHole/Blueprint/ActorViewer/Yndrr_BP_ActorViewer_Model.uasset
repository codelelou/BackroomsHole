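; Child actor viewer for inspecting an item's 3D model, adding an optional dedicated point light while the item is shown.
; An item-provided viewer scene, if valid, replaces the default, enables MoveControl and opens a gate that resets that scene's relative transform with the viewer rotation on show.
; Visibility changes toggle the camera-positioned light and temporarily enable lighting channel 1 on the item's static meshes, caching original channels for restoration on hide.
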(event `UpdateLight`
  (params (IsShow :type Boolean))
  (bind _pointlight (`self.PointLight`))
  ;[1 1 1] Light（ActorViewer用Lightが必要な場合）
  (`|ExecutionSequence`
    (:`then_0`
      (if IsShow
        (`|ExecutionSequence`
          (:`then_0`
            (`/Engine/EditorBlueprintResources/StandardMacros.DoOnce` false
              (:`Completed`
                (`LocalLightComponent.SetAttenuationRadius` _pointlight (+ (`self.CameraDistance`) 200.0)))))
          (:`then_1`
            (bind _returnvalue (`self.GetCamera`))
            (`SceneComponent.K2_SetWorldLocation` _pointlight (`SceneComponent.K2_GetComponentLocation` _returnvalue) false false))
          (:`then_2`
            (`SceneComponent.SetHiddenInGame` (`self.LightScene`) (not IsShow) true :!label _label)))
        (else
          (goto _label))))
    (:`then_1`
      (`self.UpdateLightingChannels` IsShow))))

(event `self.CallVisibilityChangedEventDispatcher`
  (params (Visibility :type Boolean))
  (`parent.CallVisibilityChangedEventDispatcher` Visibility)
  (`self.UpdateLight` Visibility))

(event `self.SetItemTransform`
  (params (Transform :type "Transform Structure"))
  (`parent.SetItemTransform` Transform))

(event `self.SetupBeginShowItem`
  (`parent.SetupBeginShowItem`)
  (`/Engine/EditorBlueprintResources/StandardMacros.Gate` true :!label _label_2
    (:`Exit`
      (bind _returnvalue (`self.GetItemScene`))
      (`SceneComponent.K2_SetRelativeTransform` _returnvalue (`KismetMathLibrary.MakeTransform` (.location (stale `self.BackupItemProperty` SceneRelativeTransform)) (.rotation (stale `self.SetItemTransform` Transform)) (.scale (stale `self.BackupItemProperty` SceneRelativeTransform))) false false))))

(event `UpdateLightingChannels`
  (params (IsShow :type Boolean))
  (bind _tmplightingchannels (`self.TmpLightingChannels`))
  ;[1 1 1] LightChannels（ActorViewer用Lightを使用する場合にItemのみに当てるためにLightChannelsを一時的に変更）
  (bind _returnvalue (`self.GetItemScene`))
  (if IsShow
    (bind _children (`SceneComponent.GetChildrenComponents` _returnvalue true))
    (for (_array_element _array_index) _children
      (`|ExecutionSequence`
        (:`then_0`
          (`/Engine/EditorBlueprintResources/StandardMacros.DoOnce` false :!label _label_3
            (:`Completed`
              (`BlueprintMapLibrary.Map_Clear` _tmplightingchannels))))
        (:`then_1`
          (bind _asstatic_mesh_component (cast `StaticMeshComponent` _array_element))
          (`|ExecutionSequence`
            (:`then_0`
              (bind _lightingchannels (`PrimitiveComponent.LightingChannels` _asstatic_mesh_component))
              (`self.AddCurrentItemLightingChannels` _array_index _lightingchannels))
            (:`then_1`
              (bind (_bchannel0 _bchannel1 _bchannel2) (break `LightingChannels` _lightingchannels))
              (`PrimitiveComponent.SetLightingChannels` _asstatic_mesh_component _bchannel0 true _bchannel2))))))
    (else
      (`|ExecutionSequence`
        (:`then_0`
          (bind _keys (`BlueprintMapLibrary.Map_Keys` _tmplightingchannels)))
        (:`then_1`
          (for (_array_element_2 _array_index_2) _children
            (if (`KismetArrayLibrary.Array_Contains` _keys _array_index_2)
              (bind _asstatic_mesh_component_2 (cast `StaticMeshComponent` _array_element_2))
              (bind (_bchannel0_2 _bchannel1_2 _bchannel2_2) (break `LightingChannels` (`BlueprintMapLibrary.Map_Find` _tmplightingchannels _array_index)))
              (`PrimitiveComponent.SetLightingChannels` _asstatic_mesh_component_2 _bchannel0_2 _bchannel1_2 _bchannel2_2))))
        (:`then_2`
          (goto _label_3 :!via `Reset`))))))

(event `self.BackupItemProperty`
  (params (ActorWorldTransform :type "Transform Structure") (SceneWorldTransform :type "Transform Structure") (SceneRelativeTransform :type "Transform Structure") (EnableCollision :type Boolean))
  (`parent.BackupItemProperty` ActorWorldTransform SceneWorldTransform SceneRelativeTransform EnableCollision))

(event `self.SetItemScene`
  (params (ItemScene :type "SceneComponent Object Reference"))
  (bind _returnvalue (message `/Game/BackroomsHole/Blueprint/Actor/Yndrr_BPI_Actor_ActorViewer_Interface.GetActorViewerSceneInActor` (`self.ItemActor`)))
  (`/Engine/EditorBlueprintResources/StandardMacros.IsValid` _returnvalue
    (:`Is Valid`
      (`|ExecutionSequence`
        (:`then_0`
          (`parent.SetItemScene` _returnvalue))
        (:`then_1`
          (set `self.MoveControl` true))
        (:`then_2`
          (goto _label_2 :!via `Open`))))
    (:`Is Not Valid`
      (`|ExecutionSequence`
        (:`then_0`
          (`parent.SetItemScene` ItemScene))
        (:`then_1`
          (goto _label_2 :!via `Close`))))))

(event `AddCurrentItemLightingChannels`
  (params (Index :type "Integer (by ref)") (LightingChannnels :type "LightingChannels Structure"))
  ;[1 1 1] LightChannels（ActorViewer用Lightを使用する場合にItemのみに当てるためにLightChannelsを一時的に変更）
  (`BlueprintMapLibrary.Map_Add` (`self.TmpLightingChannels`) Index LightingChannnels))

(fn `UserConstructionScript`
  (`parent.UserConstructionScript`))